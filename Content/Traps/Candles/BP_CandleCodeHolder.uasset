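; BP_CandleCodeHolder runs a candle-order puzzle that notifies a linked door when solved.
; On BeginPlay it registers itself with each candle in its Candles array, which doubles as the solution sequence.
; CandleAdd records candles until the count matches, then compares both arrays: a match sets IsActivated and calls the door's check event.
; A mismatch resets the candles' lights after a short delay and clears the attempt.
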(event `self.ReceiveBeginPlay`
  (for _array_element (`self.Candles`)
    (bind _asbp_candle (cast `/Game/Traps/Candles/BP_Candle` _array_element))
    (`/Game/Traps/Candles/BP_Candle.Find The Tie` _asbp_candle self)))

(event `CandleAdd`
  (params (CandleToAdd :type "/Game/Puzzle_and_Trap/PuzzleParts/BP_Lever_Parent Object Reference"))
  (`KismetArrayLibrary.Array_Append` (`self.ActiveCandles`) (`|MakeArray` CandleToAdd))
  (if (== (`KismetArrayLibrary.Array_Length` (`self.ActiveCandles`)) (`KismetArrayLibrary.Array_Length` (`self.Candles`)))
    (if (`KismetArrayLibrary.Array_Identical` (`self.ActiveCandles`) (`self.Candles`))
      (set `self.IsActivated` true)
      (`/Game/Puzzle_and_Trap/PuzzleParts/BP_Door_Parent.CallCheck_Event` (`self.ThisDoor`))
      (else
        (`KismetSystemLibrary.Delay` 0.2)
        (for _array_element (`self.ActiveCandles`)
          (bind _asbp_candle (cast `/Game/Traps/Candles/BP_Candle` _array_element))
          (`/Game/Traps/Candles/BP_Candle.ResetLight` _asbp_candle))
        (`KismetArrayLibrary.Array_Clear` (`self.ActiveCandles`))))))

(fn `UserConstructionScript`)