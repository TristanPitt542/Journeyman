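; Falling bookshelf trap that teeters until a pawn enters its damage box, then topples once after a brief delay.
; A replaying timeline rocks the pivot's pitch until the Fallen flag is set, then the Fall timeline's curve drives the pitch directly.
; When the fall finishes, it damages the player character only if it is BP_Coco and still inside the box.
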(event `self.ReceiveBeginPlay`
  (`self.Teeter`))

(event `Teeter`
  (bind (_direction _alpha) (`Timeline|TeeterTime` :!via `PlayFromStart` :!label _label)
    (:`Update`
      (if (not (`self.Fallen`))
        (`SceneComponent.K2_SetRelativeRotation` (`self.Pivot`) (`KismetMathLibrary.MakeRotator` 0.0 (`KismetMathLibrary.Lerp` -5.0 -15.0 _alpha)) false false)))
    (:`Finished`
      (if (not (`self.Fallen`))
        (goto _label :!via `PlayFromStart`)))))

(event `self.damage box.OnComponentBeginOverlap`
  (params (OverlappedComponent :type "PrimitiveComponent Object Reference") (OtherActor :type "Actor Object Reference") (OtherComp :type "PrimitiveComponent Object Reference") (OtherBodyIndex :type Integer) (bFromSweep :type Boolean) (SweepResult :type "HitResult Structure (by ref)"))
  (bind _returnvalue (`GameplayStatics.GetPlayerCharacter` 0))
  (cast `Pawn` OtherActor)
  (if (not (`self.Fallen`))
    (set `self.Fallen` true)
    (`KismetSystemLibrary.Delay` 0.2)
    (bind (_direction _alpha) (`Timeline|Fall` :!via `PlayFromStart`)
      (:`Update`
        (`SceneComponent.K2_SetRelativeRotation` (`self.Pivot`) (`KismetMathLibrary.MakeRotator` 0.0 _alpha) false false))
      (:`Finished`
        (if (`PrimitiveComponent.IsOverlappingActor` (`self.damage box`) _returnvalue)
          (bind _asbp_coco (cast `/Game/CharacterController/BP_Coco` _returnvalue))
          (`GameplayStatics.ApplyDamage` _asbp_coco (`self.Base Damage`) null null "/Script/Engine.DamageType"))))))

(fn `UserConstructionScript`)