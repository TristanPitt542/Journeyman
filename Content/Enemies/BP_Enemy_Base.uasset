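; Base enemy character that handles health, hit reactions, death and loot, with empty combat, patrol and attack events as stubs.
; Damage reports a damage event, stuns the enemy during its hit montage, updates the health bar, and on death drops coins and a chance powerup.
; Death plays a montage or destroys the actor immediately if none exists.
; Helpers drive lock-on widget visuals, trace attack range and swap mesh overlay materials by room name.
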(event `self.ReceiveAnyDamage`
  (params (Damage :type "Float (single-precision)") (DamageType :type "DamageType Object Reference") (InstigatedBy :type "Controller Object Reference") (DamageCauser :type "Actor Object Reference"))
  (`AISense_Damage.ReportDamageEvent` self DamageCauser Damage (`self.K2_GetActorLocation` DamageCauser))
  (`/Engine/EditorBlueprintResources/StandardMacros.IsValid` (`self.GetCurrentMontage`)
    (:`Is Valid`
      _)
    (:`Is Not Valid`
      (bind _returnvalue (`self.PlayAnimMontage` (`self.HitAnimation`)))
      (`self.Stunned` _returnvalue)))
  (bind _output_get (set `self.Health` (- (`self.Health`) Damage)))
  (`/Game/UI/Widgets/WBP_EnemyHealth.Set Health` (`self.As WBP Enemy Health`) _output_get)
  (if (<= _output_get 0.0)
    (`self.Drop Items` (`self.CoinsDropped`))
    (`self.Death`)))

(event `Damage Cooldown`
  ;[1 1 1] Damage Cooldown
  (set `self.bCanBeDamaged` false)
  (`KismetSystemLibrary.Delay` (`self.DamageCooldownTime`))
  (set `self.bCanBeDamaged` true))

(event `Stunned`
  (params (StunTime :type "Float (double-precision)"))
  (bind _charactermovement (`self.CharacterMovement`))
  ;[1 1 1] Stunned
  (set `self.IsStunned` true)
  (set `CharacterMovementComponent.MaxWalkSpeed` 0.0 _charactermovement)
  (`KismetSystemLibrary.Delay` StunTime)
  (set `CharacterMovementComponent.MaxWalkSpeed` (`self.AggressiveSpeed`) _charactermovement)
  (set `self.IsStunned` false))

(event `Despawn Body`
  ;[1 1 1] Death
  (`KismetSystemLibrary.Delay` 3.0)
  (`self.K2_DestroyActor` :!label _label))

(event `Exit Combat`
  ;[1 1 1] Define Events
)

(event `Patrol`
  ;[1 1 1] Define Events
)

(event `Death`
  ;[1 1 1] Death
  (`self.Hide Prompt`)
  (`self.Hide Circle`)
  (`/Game/UI/Widgets/WBP_EnemyHealth.Hide` (`self.As WBP Enemy Health`))
  (`/Engine/EditorBlueprintResources/StandardMacros.IsValid` (`self.DeathAnimation`)
    (:`Is Valid`
      (`MovementComponent.StopMovementImmediately` (`self.CharacterMovement`))
      (`Controller.UnPossess` (`self.GetController`))
      (`self.SetActorEnableCollision` false)
      (`self.PlayAnimMontage` (`self.DeathAnimation`) (`self.DeathAnimPlayRate`)))
    (:`Is Not Valid`
      (goto _label))))

(event `Enter Combat`
  ;[1 1 1] Define Events
)

(event `ChargeAttack`
  ;[1 1 1] Define Events
)

(event `PlayerInRangeCheck`
  ;[1 1 1] Define Events
)

(event `Attack`
  ;[1 1 1] Define Events
)

(event `Bind Events`
  ;[1 1 1] Define Events
)

(event `Chase Player`
  ;[1 1 1] Define Events
)

(event `self.ReceiveBeginPlay`
  (bind _as_wbp_enemy_health (`self.As WBP Enemy Health`))
  ;[1 1 1] Initialise Stuff
  (bind _returnvalue (`GameplayStatics.GetActorOfClass` "/Game/Enemies/BP_Combat_Manager.BP_Combat_Manager_C"))
  (set `self.Combat Manager` _returnvalue)
  (bind _aswbp_lock_on (cast `/Game/UI/Widgets/WBP_LockOn` (`WidgetComponent.GetWidget` (`self.Lock On`))))
  (set `self.As WBP Lock On` _aswbp_lock_on)
  (bind _aswbp_enemy_health (cast `/Game/UI/Widgets/WBP_EnemyHealth` (`WidgetComponent.GetWidget` (`self.HealthBar`))))
  (set `self.As WBP Enemy Health` _aswbp_enemy_health)
  (set `/Game/UI/Widgets/WBP_EnemyHealth.MaxHP` (`self.MaxHealth`) _as_wbp_enemy_health)
  (`/Game/UI/Widgets/WBP_EnemyHealth.Set Health` _as_wbp_enemy_health (`self.Health`))
  (set `self.AnimationBP` (`SkeletalMeshComponent.GetAnimInstance` (`self.Mesh`))))

(event `self.ReceiveActorEndOverlap`
  (params (OtherActor :type "Actor Object Reference")))

(fn `Drop Items`
  (params (Coins :type Integer))
  (bind _returnvalue (`KismetMathLibrary.Conv_VectorToTransform` (`self.K2_GetActorLocation`)))
  (for _ (range Coins)
    (`|SpawnActorFromClass` "/Game/Pickup/BP_Coin.BP_Coin_C" _returnvalue "AdjustIfPossibleButAlwaysSpawn" "MultiplyWithRoot" null false null))
  (if (== (`KismetMathLibrary.RandomInteger` 5) 0)
    (`|SpawnActorFromClass` "/Game/Pickup/BP_Powerup.BP_Powerup_C" _returnvalue "AdjustIfPossibleButAlwaysSpawn" "MultiplyWithRoot" null false null))
  (return))

(fn `Hide Circle`
  (`/Game/UI/Widgets/WBP_LockOn.Hide Circle` (`self.As WBP Lock On`)))

(fn `Hide Prompt`
  (`/Game/UI/Widgets/WBP_LockOn.Hide Prompt` (`self.As WBP Lock On`)))

(fn `Line Trace`
  (returns (`Out Hit Hit Actor` :type "Actor Object Reference"))
  (bind _returnvalue (`self.K2_GetActorLocation`))
  (bind (_returnvalue_x _returnvalue_y) (`KismetMathLibrary.BreakVector` (+ _returnvalue (* (`self.GetActorForwardVector`) (`self.AttackRange`)))))
  (bind _outhit (`KismetSystemLibrary.LineTraceSingleForObjects` _returnvalue (`KismetMathLibrary.MakeVector` _returnvalue_x _returnvalue_y (`self.Calculate Trace Z Value`)) (`|MakeArray` "ObjectTypeQuery3" :!type "EObjectTypeQuery Enum")))
  (return (`.HitActor` (`GameplayStatics.BreakHitResult` _outhit))))

(fn `NewOverlay`
  (params (`Room Entered` :type "MaterialParameterCollection Object Reference"))
  (`self.SetOverlay` (`KismetSystemLibrary.GetDisplayName` `Room Entered`)))

(fn `SetOverlay`
  (params (RoomName :type String))
  (bind _mesh (`self.Mesh`))
  (switch `string` RoomName
    (:`MPC_Foyer`
      (`MeshComponent.SetOverlayMaterial` _mesh "/Game/FadingMaterials/Foyer/M_Foyer_Overlay.M_Foyer_Overlay"))
    (:`MPC_Library`
      (`MeshComponent.SetOverlayMaterial` _mesh "/Game/FadingMaterials/Library/M_Library_Overlay.M_Library_Overlay"))
    (:`MPC_LibraryBack`
      (`MeshComponent.SetOverlayMaterial` _mesh "/Game/FadingMaterials/Library/M_LibraryBack_Overlay.M_LibraryBack_Overlay"))
    (:`MPC_Study`
      (`MeshComponent.SetOverlayMaterial` _mesh "/Game/FadingMaterials/Study/M_Study_Overlay.M_Study_Overlay"))
    (:`MPC_StudyBack`
      (`MeshComponent.SetOverlayMaterial` _mesh "/Game/FadingMaterials/Study/M_StudyBack_Overlay.M_StudyBack_Overlay"))
    (:`MPC_Throne`
      (`MeshComponent.SetOverlayMaterial` _mesh "/Game/FadingMaterials/Throne/M_Throne_Overlay.M_Throne_Overlay"))
    (:`MPC_ThroneBack`
      (`MeshComponent.SetOverlayMaterial` _mesh "/Game/FadingMaterials/Throne/M_ThroneBack_Overlay.M_ThroneBack_Overlay"))
    (:`MPC_BalconyStairs`
      (`MeshComponent.SetOverlayMaterial` _mesh "/Game/FadingMaterials/BalconyStairs/M_BalconyStairs_Overlay.M_BalconyStairs_Overlay"))
    (:`MPC_DrawingRoom`
      (`MeshComponent.SetOverlayMaterial` _mesh "/Game/FadingMaterials/DrawingRoom/M_DrawingRoom_Overlay.M_DrawingRoom_Overlay"))
    (:`MPC_WineCellar`
      (`MeshComponent.SetOverlayMaterial` _mesh "/Game/FadingMaterials/WineCellar/M_WineCellar_Overlay.M_WineCellar_Overlay"))
    (:`MPC_Stairwell`
      (`MeshComponent.SetOverlayMaterial` _mesh "/Game/FadingMaterials/Stairwell/M_Stairwell_Overlay.M_Stairwell_Overlay"))
    (:`MPC_StariwellTop`
      (`MeshComponent.SetOverlayMaterial` _mesh "/Game/FadingMaterials/Stairwell/M_StairwellTop_Overlay.M_StairwellTop_Overlay"))
    (:`MPC_Parlour`
      (`MeshComponent.SetOverlayMaterial` _mesh "/Game/FadingMaterials/Parlour/M_Parlour_Overlay.M_Parlour_Overlay"))))

(fn `Show Circle`
  (`/Game/UI/Widgets/WBP_LockOn.Show Circle` (`self.As WBP Lock On`)))

(fn `Show Prompt`
  (`/Game/UI/Widgets/WBP_LockOn.Show Prompt` (`self.As WBP Lock On`)))

(fn `UserConstructionScript`)