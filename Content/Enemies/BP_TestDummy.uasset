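; BP_TestDummy is an enemy test dummy character for checking that damage updates its health bar.
; UpdateHealthBar copies Health into the WBP_EnemyHealth widget at BeginPlay and on any damage, ignoring its ChangeAmount input.
; Damage destroys the dummy once Health drops below zero, otherwise launches it with knockback scaled by damage.
; The launch multiplies the damage causer's forward vector by the capsule's world location, so knockback varies with map position.
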(event `self.ReceiveBeginPlay`
  ;[1 1 1] Setting health bar at spawn
  (`self.UpdateHealthBar` 0.0))

(event `self.ReceiveAnyDamage`
  (params (Damage :type "Float (single-precision)") (DamageType :type "DamageType Object Reference") (InstigatedBy :type "Controller Object Reference") (DamageCauser :type "Actor Object Reference"))
  ;[1 1 1] Test for health bar updating
  (bind _output_get (set `self.Knockback` (/ Damage 12.0)))
  (set `self.Health` (- (`self.Health`) Damage))
  (`self.UpdateHealthBar` 0.0)
  (if (< (`self.Health`) 0.0)
    (`self.K2_DestroyActor`)
    (else
      (`self.LaunchCharacter` (* (`self.GetActorForwardVector` DamageCauser) (`SceneComponent.K2_GetComponentLocation` (`self.CapsuleComponent`)) _output_get)))))

(fn `UpdateHealthBar`
  (params (ChangeAmount :type "Float (double-precision)"))
  (bind _aswbp_enemy_health (cast `/Game/UI/Widgets/WBP_EnemyHealth` (`WidgetComponent.GetUserWidgetObject` (`self.Health Bar`))))
  (set `/Game/UI/Widgets/WBP_EnemyHealth.HP` (`self.Health`) _aswbp_enemy_health)
  (return))

(fn `UserConstructionScript`)