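; Combat manager that coordinates melee enemies so they take turns attacking.
; Enter and exit events maintain a list of enemies tagged Melee; on entry, the first one found mid-attack has its CanAttack cleared.
; An attack start clears CanAttack on every other listed enemy, and its completion restores theirs and shuffles the list.
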(event `Enemy Attacking`
  (params (`Attacking Enemy` :type "Actor Object Reference"))
  ;[1 1 1] Disables attacking for other enemies once enemy attack begins
  (for _array_element (`self.MeleeEnemiesInCombat`)
    (if (not (== _array_element `Attacking Enemy`))
      (set `/Game/Enemies/BP_Enemy_Base.CanAttack` false (cast `/Game/Enemies/BP_Enemy_Base` _array_element :!pure true)))))

(event `Enemy Enter Combat`
  (params (Enemy :type "Actor Object Reference"))
  (bind _meleeenemiesincombat (`self.MeleeEnemiesInCombat`))
  ;[1 1 1] Updates array when enemy enters/exits combat
  (if (`self.ActorHasTag` Enemy "Melee")
    (`KismetArrayLibrary.Array_AddUnique` _meleeenemiesincombat Enemy)
    (for _array_element _meleeenemiesincombat
      (bind _asbp_enemy_base (cast `/Game/Enemies/BP_Enemy_Base` _array_element :!pure true))
      (if (`/Game/Enemies/BP_Enemy_Base.IsAttacking` _asbp_enemy_base)
        (set `/Game/Enemies/BP_Enemy_Base.CanAttack` false _asbp_enemy_base)
        (break)))))

(event `Enemy Exit Combat`
  (params (Enemy :type "Actor Object Reference"))
  ;[1 1 1] Updates array when enemy enters/exits combat
  (if (`self.ActorHasTag` Enemy "Melee")
    (`KismetArrayLibrary.Array_RemoveItem` (`self.MeleeEnemiesInCombat`) Enemy)))

(event `Enemy Attack Complete`
  (params (`Attacking Enemy` :type "Actor Object Reference"))
  ;[1 1 1] Enables attacking for other enemies once enemy attack finished
  (for _array_element (`self.MeleeEnemiesInCombat`)
    (if (not (== _array_element `Attacking Enemy`))
      (set `/Game/Enemies/BP_Enemy_Base.CanAttack` true (cast `/Game/Enemies/BP_Enemy_Base` _array_element :!pure true))))
  (`KismetArrayLibrary.Array_Shuffle` (`self.MeleeEnemiesInCombat`)))

(event `self.ReceiveBeginPlay`
  ;[1 1 1] Initialises stuff
  (set `self.PlayerCharacter` (`GameplayStatics.GetPlayerCharacter` 0)))

(fn `UserConstructionScript`)