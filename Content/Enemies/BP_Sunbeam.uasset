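; BP_Sunbeam is a timed enemy beam hazard that drains the player's (BP_Coco) stamina on contact.
; It configures a Niagara beam's width and end point, refreshes the end on a looping timer, and calls BeamExpired before destroying itself after its lifespan.
; Exported Niagara particle data drives small sphere traces; a player hit reduces stamina, stops regeneration, updates the UI and calls StaminaDrained.
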(event `UpdateBeam`
  ;[1 1 1] Update Beam
  (`NiagaraComponent.SetVariableVec3` (`self.Beam`) "Beam End" (`self.BeamEnd`)))

(event `self.ReceiveBeginPlay`
  (bind _beam (`self.Beam`))
  ;[1 1 1] Initialise stuff
  (`NiagaraComponent.SetVariableFloat` _beam "Beam Width" (`self.BeamWidth`))
  (`NiagaraComponent.SetVariableVec3` _beam "Beam End" (`self.BeamEnd`))
  (`NiagaraComponent.SetVariableObject` _beam "BeamBP" self)
  (`KismetSystemLibrary.K2_SetTimerDelegate` (delegate `UpdateBeam`) 0.05 true)
  (`KismetSystemLibrary.Delay` (`self.Lifespan`))
  (`self.Beam Expired`)
  (`self.K2_DestroyActor`))

(event `Drain Stamina`
  (bind _asbp_coco (cast `/Game/CharacterController/BP_Coco` (`GameplayStatics.GetPlayerCharacter` 0) :!pure true))
  ;[1 1 1] Drain Stamina
  (bind _output_get (set `/Game/CharacterController/BP_Coco.Stamina` (- (`/Game/CharacterController/BP_Coco.Stamina` _asbp_coco) (`self.StaminaDrainAmount`)) _asbp_coco))
  (set `/Game/CharacterController/BP_Coco.ShouldRegen` false _asbp_coco)
  (`/Game/UI/Widgets/BP_UI.Set Stamina` (`/Game/CharacterController/BP_Coco.UI` _asbp_coco) _output_get)
  (`/Game/CharacterController/BP_Coco.Stamina Drained` _asbp_coco))

(event `self.ReceiveParticleData`
  (params (Data :type "Array of BasicParticleData Structure (by ref)") (NiagaraSystem :type "NiagaraSystem Object Reference") (SimulationPositionOffset :type "Vector Structure (by ref)"))
  ;[1 1 1] Receives data from niagara collision
  (for _array_element Data
    (bind _position (break `BasicParticleData` _array_element))
    (bind _outhit (`KismetSystemLibrary.SphereTraceSingleForObjects` _position _position 20.0 (`|MakeArray` "ObjectTypeQuery3" :!type "EObjectTypeQuery Enum")))
    (if (== (`.HitActor` (`GameplayStatics.BreakHitResult` _outhit)) (`GameplayStatics.GetPlayerCharacter` 0))
      (`self.Drain Stamina`)
      (break))))

(fn `UserConstructionScript`)