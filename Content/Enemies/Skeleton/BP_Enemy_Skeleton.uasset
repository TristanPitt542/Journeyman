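; Skeleton enemy that runs a behavior tree and implements patrol, chase, combat entry/exit and melee attack events.
; Attacks charge up, lunge on a looping timer, swing a montage on arrival or timeout, then retreat and cool down.
; DealDamage applies damage through a forward sphere trace and starts the retreat.
; Combat and attack states are reported to CombatManager, with an indicator material showing the current phase.
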(event `self.Death`
  (bind _combat_manager (`self.Combat Manager`))
  (if (`self.IsAttacking`)
    (`/Game/Enemies/BP_Combat_Manager.Enemy Attack Complete` _combat_manager self)
    (`/Game/Enemies/BP_Combat_Manager.Enemy Exit Combat` _combat_manager self)
    (set `self.CanAttack` false))
  (`parent.Death`))

(event `self.ReceiveBeginPlay`
  ;[1 1 1] Initialises stuff
  (`AIController.RunBehaviorTree` (`AIBlueprintHelperLibrary.GetAIController` self) "/Game/Enemies/Skeleton/BT_Skeleton.BT_Skeleton")
  (set `self.BaseLocation` (`self.K2_GetActorLocation`))
  (set `CharacterMovementComponent.MaxWalkSpeed` (`self.PassiveSpeed`) (`self.CharacterMovement`))
  (`parent.ReceiveBeginPlay`))

(event `Skip Attack`
  ;[1 1 1] Attack
  ;;[1 1 1] Attack Complete
  (`self.AttackComplete` :!label _label)
  (`PrimitiveComponent.SetMaterial` (`self.AttackIndicator`) 0 "/Game/Enemies/TestStuff/M_TestMaterial_Yellow.M_TestMaterial_Yellow")
  (set `self.IsAttacking` false))

(event `Lunge`
  ;[1 1 1] Attack
  ;;[1 1 1] Move to player to attack
  (`|AIMoveTo` self (`self.K2_GetActorLocation` (`GameplayStatics.GetPlayerCharacter` 0)) null 150.0
    (:`OnSuccess`
      (`self.Swing`))))

(event `FinishAttackCycle`
  ;[1 1 1] Attack
  ;;[1 1 1] Attack Complete
  (if (`self.Retreating`)
    (set `self.Retreating` false)
    (`KismetSystemLibrary.Delay` (`self.CooldownTime`))
    (`/Game/Enemies/BP_Combat_Manager.Enemy Attack Complete` (`self.Combat Manager`) self)
    (`AIController.K2_ClearFocus` (`AIBlueprintHelperLibrary.GetAIController` self))
    (goto _label)))

(event `self.Enter Combat`
  ;[1 1 1] Handles entering + exiting combat
  (`PrimitiveComponent.SetMaterial` (`self.AttackIndicator`) 0 "/Game/Enemies/TestStuff/M_TestMaterial_Yellow.M_TestMaterial_Yellow")
  (set `self.InCombat` true)
  (set `CharacterMovementComponent.MaxWalkSpeed` (`self.AggressiveSpeed`) (`self.CharacterMovement`))
  (`self.EnterCombat`)
  (`/Game/Enemies/BP_Combat_Manager.Enemy Enter Combat` (`self.Combat Manager`) self))

(event `self.Attack`
  ;[1 1 1] Attack
  ;;[1 1 1] Begin Attack Process
  (if (`self.CanAttack`)
    (`self.InitialiseAttack`)
    (`KismetSystemLibrary.Delay` (`self.AttackChargeTime`))
    (set `self.AttackTriggered` false)
    (bind _returnvalue (`KismetSystemLibrary.K2_SetTimerDelegate` (delegate `Lunge`) 0.05 true))
    (`KismetSystemLibrary.Delay` 1.0)
    (`self.Swing`)
    (else
      (`self.Skip Attack`))))

(event `Deal Damage`
  ;[1 1 1] Attack
  ;;[1 1 1] Do Trace + Deal Damage
  (`self.Damage Trace`)
  (`KismetSystemLibrary.Delay` 0.5)
  (`AIController.K2_SetFocus` (`AIBlueprintHelperLibrary.GetAIController` self) (`GameplayStatics.GetPlayerCharacter` 0))
  (bind _returnvalue (`KismetSystemLibrary.K2_SetTimerDelegate` (delegate `Retreat`) 0.05 true))
  (set `self.Retreating` true)
  (`KismetSystemLibrary.Delay` 1.0)
  (`KismetSystemLibrary.K2_ClearAndInvalidateTimerHandle` _returnvalue)
  (`self.FinishAttackCycle`))

(event `self.Exit Combat`
  ;[1 1 1] Handles entering + exiting combat
  (`PrimitiveComponent.SetMaterial` (`self.AttackIndicator`) 0 "/Game/Enemies/TestStuff/M_TestMaterial_Green.M_TestMaterial_Green")
  (set `self.InCombat` false)
  (set `CharacterMovementComponent.MaxWalkSpeed` (`self.PassiveSpeed`) (`self.CharacterMovement`))
  (`self.ExitCombat`)
  (`/Game/Enemies/BP_Combat_Manager.Enemy Exit Combat` (`self.Combat Manager`) self))

(event `Retreat`
  ;[1 1 1] Attack
  ;;[1 1 1] Retreat After Attack
  (if (< (`self.GetDistanceTo` (`GameplayStatics.GetPlayerCharacter` 0)) (`self.BeginAttackRange`))
    (`self.Move Out Of Range`)
    (else
      (`KismetSystemLibrary.K2_ClearAndInvalidateTimerHandle` (stale `Deal Damage` _returnvalue))
      (`self.FinishAttackCycle`))))

(event `Swing`
  ;[1 1 1] Attack
  ;;[1 1 1] Attack Animation
  (if (not (or (`self.AttackTriggered`) (not (`self.CanAttack`))))
    (set `self.AttackTriggered` true)
    (`KismetSystemLibrary.K2_ClearAndInvalidateTimerHandle` (stale `self.Attack` _returnvalue))
    (`PrimitiveComponent.SetMaterial` (`self.AttackIndicator`) 0 "/Game/Enemies/TestStuff/M_TestMaterial_Red.M_TestMaterial_Red")
    (`AIController.K2_ClearFocus` (`AIBlueprintHelperLibrary.GetAIController` self))
    (`self.PlayAnimMontage` "/Game/Enemies/Skeleton/Animations/AM_SkeletonAttack.AM_SkeletonAttack")))

(event `self.Patrol`
  ;[1 1 1] Enemy patrolling
  (`|AIMoveTo` self (`NavigationSystemV1.K2_GetRandomReachablePointInRadius` (`self.BaseLocation`) (`self.PatrolRadius`) null null) null
    (:`OnSuccess`
      (`self.PatrolComplete`))))

(event `self.Chase Player`
  ;[1 1 1] Enemy chasing player
  (`|AIMoveTo` self (`self.K2_GetActorLocation` (`GameplayStatics.GetPlayerCharacter` 0)) null (`self.BeginAttackRange`)
    (:`OnSuccess`
      (`self.BeginAttack`))))

(fn `Damage Trace`
  (bind _returnvalue (`self.K2_GetActorLocation`))
  (bind _outactors (`GameplayStatics.GetAllActorsOfClass` "/Script/Engine.TriggerVolume"))
  (bind _outhit (`KismetSystemLibrary.SphereTraceSingleForObjects` _returnvalue (+ _returnvalue (* (`self.GetActorForwardVector`) (`self.AttackRange`))) 30.0 (`|MakeArray` "ObjectTypeQuery3" "ObjectTypeQuery1" :!type "EObjectTypeQuery Enum") false _outactors))
  (`GameplayStatics.ApplyDamage` (`.HitActor` (`GameplayStatics.BreakHitResult` _outhit)) (`self.Damage`) null null "/Script/Engine.DamageType"))

(fn `InitialiseAttack`
  (`PrimitiveComponent.SetMaterial` (`self.AttackIndicator`) 0 "/Game/Enemies/TestStuff/M_TestMaterial_Orange.M_TestMaterial_Orange")
  (set `self.IsAttacking` true)
  (`/Game/Enemies/BP_Combat_Manager.Enemy Attacking` (`self.Combat Manager`) self)
  (`AIController.K2_SetFocus` (`AIBlueprintHelperLibrary.GetAIController` self) (`GameplayStatics.GetPlayerCharacter` 0))
  (return))

(fn `Move Out Of Range`
  (`AIController.MoveToLocation` (`AIBlueprintHelperLibrary.GetAIController` self) (+ (`self.K2_GetActorLocation`) (* (`self.GetActorForwardVector`) -50.0)) 0.0 true true false true null true))

(fn `UserConstructionScript`
  (`parent.UserConstructionScript`))