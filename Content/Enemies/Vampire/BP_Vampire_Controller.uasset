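; AI controller for the vampire enemy that switches it in and out of combat based on perception of the player.
; BeginPlay caches the controlled pawn as BP_Enemy_Vampire, and perception updates for player 0 call its EnterCombat or ExitCombat.
; Combat exit is skipped while the vampire is attacking or the player is within a hard-coded distance, which must stay slightly below the lose sight radius.
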(event `self.AIPerception.OnTargetPerceptionUpdated`
  (params (Actor :type "Actor Object Reference") (Stimulus :type "AIStimulus Structure"))
  (bind _returnvalue (`GameplayStatics.GetPlayerCharacter` 0))
  (bind _enemy (`self.Enemy`))
  (if (== Actor _returnvalue)
    (if Stimulus_bSuccessfullySensed
      (if (not (`/Game/Enemies/BP_Enemy_Base.InCombat` _enemy))
        (set `/Game/Enemies/BP_Enemy_Base.InCombat` true _enemy)
        (`/Game/Enemies/BP_Enemy_Base.Enter Combat` _enemy))
      (elif (not (or (`/Game/Enemies/BP_Enemy_Base.IsAttacking` _enemy) (< (`self.GetDistanceTo` _returnvalue) 1195.0)))
        (`/Game/Enemies/BP_Enemy_Base.Exit Combat` _enemy)))))

(event `self.ReceiveBeginPlay`
  (set `self.Enemy` (cast `/Game/Enemies/Vampire/BP_Enemy_Vampire` (`self.K2_GetPawn`) :!pure true)))

(fn `UserConstructionScript`)