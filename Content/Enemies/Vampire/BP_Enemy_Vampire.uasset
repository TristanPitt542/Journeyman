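; Vampire enemy that runs BT_Vampire, with events for patrol, chase, combat state and attacks.
; Attack picks by distance between a push, a cooldown-gated dash and blood magic (lance, lobbed orb or three-dagger spread).
; A dash hit latches onto the player, slowing them, disabling lock-on and dealing timed damage until damaged or timed out.
; The perception handler is empty; its combat-switching logic sits disconnected.
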(event `Grabbed`
  (`GameplayStatics.ApplyDamage` (`GameplayStatics.GetPlayerCharacter` 0) 1.0))

(event `self.ReceiveAnyDamage`
  (params (Damage :type "Float (single-precision)") (DamageType :type "DamageType Object Reference") (InstigatedBy :type "Controller Object Reference") (DamageCauser :type "Actor Object Reference"))
  (`parent.ReceiveAnyDamage` Damage DamageType InstigatedBy DamageCauser)
  (if (`self.Latched`)
    (`self.End Grabbed`)))

(event `self.CapsuleComponent.OnComponentHit`
  (params (HitComponent :type "PrimitiveComponent Object Reference") (OtherActor :type "Actor Object Reference") (OtherComp :type "PrimitiveComponent Object Reference") (NormalImpulse :type "Vector Structure") (Hit :type "HitResult Structure (by ref)"))
  (if (and (== OtherActor (`GameplayStatics.GetPlayerCharacter` 0)) (`self.IsDashing`))
    (`self.K2_AttachToActor` OtherActor "None" "KeepWorld" "KeepRelative" "KeepRelative" false)
    (`MovementComponent.StopMovementImmediately` (`self.CharacterMovement`))
    (set `self.Latched` true)
    (set `CharacterMovementComponent.MaxWalkSpeed` 100.0 (`Character.CharacterMovement` (`GameplayStatics.GetPlayerCharacter` 0)))
    (`/Game/CharacterController/BP_Coco.DisengageLockOn` (cast `/Game/CharacterController/BP_Coco` (`GameplayStatics.GetPlayerCharacter` 0) :!pure true))
    (set `/Game/CharacterController/BP_Coco_Controller.CanLockOn` false (cast `/Game/CharacterController/BP_Coco_Controller` (`GameplayStatics.GetPlayerController` 0) :!pure true))
    (bind _returnvalue (`KismetSystemLibrary.K2_SetTimerDelegate` (delegate `Grabbed`) 0.2 true))
    (`KismetSystemLibrary.Delay` (`self.LatchedDuration`))
    (if (`self.Latched`)
      (`self.End Grabbed`))))

(event `End Grabbed`
  (`KismetSystemLibrary.K2_ClearAndInvalidateTimerHandle` (stale `self.CapsuleComponent.OnComponentHit` _returnvalue))
  (set `self.Latched` false)
  (`self.K2_DetachFromActor` "KeepWorld" "KeepWorld" "KeepWorld")
  (`self.LaunchCharacter` (* (`self.GetActorForwardVector`) -2000.0))
  (set `CharacterMovementComponent.MaxWalkSpeed` 600.0 (`Character.CharacterMovement` (`GameplayStatics.GetPlayerCharacter` 0)))
  (set `/Game/CharacterController/BP_Coco_Controller.CanLockOn` true (cast `/Game/CharacterController/BP_Coco_Controller` (`GameplayStatics.GetPlayerController` 0) :!pure true))
  ;[1 1 1] Vampire dash attack functionality
  (`self.PlayAnimMontage` "/Game/Enemies/VampireLord/Animations/AM_VampireLord_MeleeAttack.AM_VampireLord_MeleeAttack" 1.0 "Swing" :!label _label)
  (`self.Dash Cooldown`)
  (`KismetSystemLibrary.Delay` 1.0)
  (`self.AttackComplete`)
  (`PrimitiveComponent.SetMaterial` (`self.AttackIndicator`) 0 "/Game/Enemies/TestStuff/M_TestMaterial_Yellow.M_TestMaterial_Yellow")
  (set `self.IsAttacking` false))

(event `Dash Attack`
  (`self.PlayAnimMontage` "/Game/Enemies/VampireLord/Animations/AM_VampireLord_MeleeAttack.AM_VampireLord_MeleeAttack" 0.6))

(event `Begin Dash`
  ;[1 1 1] Vampire dash attack functionality
  (set `self.IsDashing` true)
  (`self.LaunchCharacter` (* (`self.GetActorForwardVector`) (`self.DashDistance`)))
  (`KismetSystemLibrary.Delay` 0.1)
  (set `self.IsDashing` false)
  (if (not (`self.Latched`))
    (goto _label)))

(event `self.AIPerception.OnTargetPerceptionUpdated`
  (params (Actor :type "Actor Object Reference") (Stimulus :type "AIStimulus Structure"))
  ;[1 1 1] Handles AI sensing of player
)

(event `Push Attack`
  (bind _returnvalue (`self.K2_GetActorLocation`))
  ;[1 1 1] Vampire push attack functionality
  (`KismetSystemLibrary.Delay` 0.5)
  (`KismetSystemLibrary.SphereTraceSingle` _returnvalue (+ _returnvalue (* (`self.GetActorForwardVector`) (`self.PushRange`))) 30.0 "TraceTypeQuery1")
  (`self.LaunchCharacter` (`GameplayStatics.GetPlayerCharacter` 0) (* (`self.GetActorForwardVector`) (`self.PushPower`)) false false)
  (`KismetSystemLibrary.Delay` 1.5)
  (`self.AttackComplete`)
  (`PrimitiveComponent.SetMaterial` (`self.AttackIndicator`) 0 "/Game/Enemies/TestStuff/M_TestMaterial_Yellow.M_TestMaterial_Yellow")
  (set `self.IsAttacking` false))

(event `self.ReceiveBeginPlay`
  ;[1 1 1] Initialises stuff
  (`AIController.RunBehaviorTree` (`AIBlueprintHelperLibrary.GetAIController` self) "/Game/Enemies/Vampire/BT_Vampire.BT_Vampire")
  (set `self.BaseLocation` (`self.K2_GetActorLocation`))
  (set `CharacterMovementComponent.MaxWalkSpeed` (`self.PassiveSpeed`) (`self.CharacterMovement`))
  (`parent.ReceiveBeginPlay`))

(event `Dash Cooldown`
  ;[1 1 1] Dash cooldown
  (set `self.CanDash` false)
  (`KismetSystemLibrary.Delay` (`self.DashCooldown`))
  (set `self.CanDash` true))

(event `self.Enter Combat`
  ;[1 1 1] Handles entering + exiting combat
  (`PrimitiveComponent.SetMaterial` (`self.AttackIndicator`) 0 "/Game/Enemies/TestStuff/M_TestMaterial_Yellow.M_TestMaterial_Yellow")
  (set `self.InCombat` true)
  (set `CharacterMovementComponent.MaxWalkSpeed` (`self.AggressiveSpeed`) (`self.CharacterMovement`))
  (`self.EnterCombat`))

(event `Magic Attack`
  ;[1 1 1] Vampire magic attack - chooses which to use then uses it - changes attack type afterwards if random attacks enabled
  (`self.PlayAnimMontage` "/Game/Enemies/VampireLord/Animations/AM_VampireLord_MagicAttack.AM_VampireLord_MagicAttack"))

(event `self.Exit Combat`
  ;[1 1 1] Handles entering + exiting combat
  (`PrimitiveComponent.SetMaterial` (`self.AttackIndicator`) 0 "/Game/Enemies/TestStuff/M_TestMaterial_Green.M_TestMaterial_Green")
  (set `self.InCombat` false)
  (set `CharacterMovementComponent.MaxWalkSpeed` (`self.PassiveSpeed`) (`self.CharacterMovement`))
  (`self.ExitCombat`))

(event `Choose Attack`
  (bind _returnvalue (`SceneComponent.K2_GetComponentLocation` (`self.ProjectileSpawn`)))
  ;[1 1 1] Vampire magic attack - chooses which to use then uses it - changes attack type afterwards if random attacks enabled
  (switch `int` (`self.AttackType`)
    (:`0`
      (`PrimitiveComponent.SetMaterial` (`self.AttackIndicator`) 0 "/Game/Enemies/TestStuff/M_TestMaterial_Red.M_TestMaterial_Red")
      (`|SpawnActorFromClass` "/Game/Enemies/Projectiles/BP_Vampire_Blood_Lance.BP_Vampire_Blood_Lance_C" (`KismetMathLibrary.MakeTransform` _returnvalue (`KismetMathLibrary.FindLookAtRotation` _returnvalue (`self.K2_GetActorLocation` (`GameplayStatics.GetPlayerCharacter` 0)))) "Undefined" "MultiplyWithRoot" null 7.5 1500.0 self null))
    (:`1`
      (`PrimitiveComponent.SetMaterial` (`self.AttackIndicator`) 0 "/Game/Enemies/TestStuff/M_TestMaterial_Red.M_TestMaterial_Red")
      (`self.AOE Attack`))
    (:`2`
      (`PrimitiveComponent.SetMaterial` (`self.AttackIndicator`) 0 "/Game/Enemies/TestStuff/M_TestMaterial_Red.M_TestMaterial_Red")
      (`self.3ShotAttack`)))
  (if (`self.RandomMagicAttacks`)
    (set `self.AttackType` (`KismetMathLibrary.RandomInteger` 3)))
  (`KismetSystemLibrary.Delay` 1.5)
  (`self.AttackComplete`)
  (`PrimitiveComponent.SetMaterial` (`self.AttackIndicator`) 0 "/Game/Enemies/TestStuff/M_TestMaterial_Yellow.M_TestMaterial_Yellow")
  (set `self.IsAttacking` false))

(event `self.Patrol`
  ;[1 1 1] Enemy patrolling
  (`|AIMoveTo` self (`NavigationSystemV1.K2_GetRandomReachablePointInRadius` (`self.BaseLocation`) (`self.PatrolRadius`) null null) null
    (:`OnSuccess`
      (`self.PatrolComplete`))))

(event `self.Chase Player`
  ;[1 1 1] Enemy chasing player
  (`|AIMoveTo` self (`self.K2_GetActorLocation` (`GameplayStatics.GetPlayerCharacter` 0)) null (`self.BeginAttackRange`)
    (:`OnSuccess`
      (`self.BeginAttack`))))

(event `self.Attack`
  (bind _returnvalue (`self.GetDistanceTo` (`GameplayStatics.GetPlayerCharacter` 0)))
  ;[1 1 1] Enemy attack decision logic
  (`PrimitiveComponent.SetMaterial` (`self.AttackIndicator`) 0 "/Game/Enemies/TestStuff/M_TestMaterial_Orange.M_TestMaterial_Orange")
  (set `self.IsAttacking` true)
  (if (< _returnvalue (`self.PushRange`))
    (`self.Push Attack`)
    (elif (and (< _returnvalue (`self.DashAttackRange`)) (`self.CanDash`))
      (`self.Dash Attack`)
      (else
        (`self.Magic Attack`)))))

(fn `3ShotAttack`
  (bind _returnvalue (`SceneComponent.K2_GetComponentLocation` (`self.ProjectileSpawn`)))
  (bind _returnvalue_2 (`SceneComponent.K2_GetComponentLocation` (`self.ProjectileSpawn`)))
  (bind _returnvalue_3 (`SceneComponent.K2_GetComponentLocation` (`self.ProjectileSpawn`)))
  (bind (_returnvalue_roll _returnvalue_pitch _returnvalue_yaw) (`KismetMathLibrary.BreakRotator` (`KismetMathLibrary.FindLookAtRotation` _returnvalue_2 (`self.K2_GetActorLocation` (`GameplayStatics.GetPlayerCharacter` 0)))))
  (bind (_returnvalue_roll_2 _returnvalue_pitch_2 _returnvalue_yaw_2) (`KismetMathLibrary.BreakRotator` (`KismetMathLibrary.FindLookAtRotation` _returnvalue (`self.K2_GetActorLocation` (`GameplayStatics.GetPlayerCharacter` 0)))))
  (`|SpawnActorFromClass` "/Game/Enemies/Projectiles/BP_Vampire_Blood_Dagger.BP_Vampire_Blood_Dagger_C" (`KismetMathLibrary.MakeTransform` _returnvalue_2 (`KismetMathLibrary.MakeRotator` _returnvalue_roll _returnvalue_pitch (- _returnvalue_yaw 30.0))) "Undefined" "MultiplyWithRoot" null 5.0 750.0 self null)
  (`|SpawnActorFromClass` "/Game/Enemies/Projectiles/BP_Vampire_Blood_Dagger.BP_Vampire_Blood_Dagger_C" (`KismetMathLibrary.MakeTransform` _returnvalue_3 (`KismetMathLibrary.FindLookAtRotation` _returnvalue_3 (`self.K2_GetActorLocation` (`GameplayStatics.GetPlayerCharacter` 0)))) "Undefined" "MultiplyWithRoot" null 5.0 750.0 self null)
  (`|SpawnActorFromClass` "/Game/Enemies/Projectiles/BP_Vampire_Blood_Dagger.BP_Vampire_Blood_Dagger_C" (`KismetMathLibrary.MakeTransform` _returnvalue (`KismetMathLibrary.MakeRotator` _returnvalue_roll_2 _returnvalue_pitch_2 (+ _returnvalue_yaw_2 30.0))) "Undefined" "MultiplyWithRoot" null 5.0 750.0 self null))

(fn `AOE Attack`
  (bind _returnvalue (`SceneComponent.K2_GetComponentLocation` (`self.ProjectileSpawn`)))
  (bind _returnvalue_2 (`self.K2_GetActorLocation` (`GameplayStatics.GetPlayerCharacter` 0)))
  (bind _returnvalue_3 (`|SpawnActorFromClass` "/Game/Enemies/Projectiles/BP_Vampire_Blood_Orb.BP_Vampire_Blood_Orb_C" (`KismetMathLibrary.MakeTransform` _returnvalue (`KismetMathLibrary.FindLookAtRotation` _returnvalue _returnvalue_2)) "Undefined" "MultiplyWithRoot" null 10.0 1000.0 self null))
  (bind _tossvelocity (`GameplayStatics.BlueprintSuggestProjectileVelocity` _returnvalue _returnvalue_2 1000.0 0.0 "DoNotTrace" 0.0 true))
  (`PrimitiveComponent.AddImpulse` (`/Game/Enemies/Projectiles/BP_Projectile_Base.Root` _returnvalue_3) _tossvelocity "None" true))

(fn `UserConstructionScript`
  (`SceneComponent.K2_AttachToComponent` (`self.ProjectileSpawn`) (`self.Mesh`) "jnt_rightthumb" "SnapToTarget" "SnapToTarget" "KeepRelative" true)
  (`parent.UserConstructionScript`))