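; Base enemy projectile that deals damage on hit and expires after a set lifespan.
; On BeginPlay it sets the movement component's initial speed, ignores its originating enemy while moving, and starts the self-destruct delay.
; A root hit on anything but that enemy destroys it, first damaging the player character or actors whose class is exactly BP_Enemy_Base, excluding subclasses.
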(event `self.ReceiveBeginPlay`
  (set `ProjectileMovementComponent.InitialSpeed` (`self.Speed`) (`self.ProjectileMovement`))
  (`PrimitiveComponent.IgnoreActorWhenMoving` (`self.Root`) (`self.EnemyOrigin`) true)
  (`KismetSystemLibrary.Delay` (`self.ProjectileLifespan`))
  (`self.K2_DestroyActor`))

(event `self.Root.OnComponentHit`
  (params (HitComponent :type "PrimitiveComponent Object Reference") (OtherActor :type "Actor Object Reference") (OtherComp :type "PrimitiveComponent Object Reference") (NormalImpulse :type "Vector Structure") (Hit :type "HitResult Structure (by ref)"))
  (if (not (== OtherActor (`self.EnemyOrigin`)))
    (if (or (== OtherActor (`GameplayStatics.GetPlayerCharacter` 0)) (== (`GameplayStatics.GetObjectClass` OtherActor) "/Game/Enemies/BP_Enemy_Base.BP_Enemy_Base_C"))
      (`GameplayStatics.ApplyDamage` OtherActor (`self.Damage`) null self))
    (`self.K2_DestroyActor`)))

(fn `UserConstructionScript`)