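; BP_Vampire_Blood_Orb is an enemy projectile that deals radial damage on impact.
; When its Root component hits anything other than EnemyOrigin, it destroys itself.
; If that actor is the player character or exactly of class BP_Enemy_Base, it first applies radial damage around itself using its Damage and DamageType.
; The class test is an equality check, so subclasses of BP_Enemy_Base do not trigger damage.
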(event `self.Root.OnComponentHit`
  (params (HitComponent :type "PrimitiveComponent Object Reference") (OtherActor :type "Actor Object Reference") (OtherComp :type "PrimitiveComponent Object Reference") (NormalImpulse :type "Vector Structure") (Hit :type "HitResult Structure (by ref)"))
  (if (not (== OtherActor (`self.EnemyOrigin`)))
    (if (or (== OtherActor (`GameplayStatics.GetPlayerCharacter` 0)) (== (`GameplayStatics.GetObjectClass` OtherActor) "/Game/Enemies/BP_Enemy_Base.BP_Enemy_Base_C"))
      (`GameplayStatics.ApplyRadialDamage` :`BaseDamage` (`self.Damage`) :`Origin` (`self.K2_GetActorLocation`) :`DamageRadius` 200.0 :`DamageTypeClass` "/Script/Engine.DamageType" :`DamageCauser` null :`InstigatedByController` null))
    (`self.K2_DestroyActor`)))

(fn `UserConstructionScript`
  (`parent.UserConstructionScript`))