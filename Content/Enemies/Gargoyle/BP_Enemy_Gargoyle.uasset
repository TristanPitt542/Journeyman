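; Gargoyle enemy that runs a behavior tree and attacks the player with an aimed sunbeam.
; AI perception enters combat on sighting and exits on sight loss unless attacking or nearby, easing back to its default rotation.
; Attack spawns an attached BP_Sunbeam, using a looping timer to update pitch and line-traced endpoint until it expires.
; Combat, charge and attack stages fire dispatchers, with an indicator material showing state by color.
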(event `self.ReceiveTick`
  (params (DeltaSeconds :type "Float (single-precision)")))

(event `self.AIPerception.OnTargetPerceptionUpdated`
  (params (Actor :type "Actor Object Reference") (Stimulus :type "AIStimulus Structure"))
  (bind _returnvalue (`GameplayStatics.GetPlayerCharacter` 0))
  ;[1 1 1] Handles AI sensing of player
  (if (== Actor _returnvalue)
    (if Stimulus_bSuccessfullySensed
      (if (not (`self.InCombat`))
        (set `self.InCombat` true)
        (`self.Enter Combat`))
      (elif (not (or (`self.IsAttacking`) (< (`self.GetDistanceTo` _returnvalue) 995.0)))
        (`self.Exit Combat`)))))

(event `Attack Complete`
  ;[1 1 1] Enemy attack functionality
  (`KismetSystemLibrary.K2_ClearAndInvalidateTimerHandle` (stale `self.Attack` _returnvalue))
  (`self.AttackComplete`)
  (`PrimitiveComponent.SetMaterial` (`self.AttackIndicator`) 0 "/Game/Enemies/TestStuff/M_TestMaterial_Yellow.M_TestMaterial_Yellow")
  (set `self.IsAttacking` false))

(event `self.Attack`
  ;[1 1 1] Enemy attack functionality
  (set `self.IsAttacking` true)
  (`PrimitiveComponent.SetMaterial` (`self.AttackIndicator`) 0 "/Game/Enemies/TestStuff/M_TestMaterial_Red.M_TestMaterial_Red")
  (bind _sunbeam (`self.Shoot`))
  (add `/Game/Enemies/BP_Sunbeam.Beam Expired` _sunbeam (delegate `Attack Complete`))
  (bind _returnvalue (`KismetSystemLibrary.K2_SetTimerDelegate` (delegate `Update Aim`) 0.05 true)))

(event `Update Aim`
  (bind (_returnvalue_roll _returnvalue_pitch) (`KismetMathLibrary.BreakRotator` (`KismetMathLibrary.FindLookAtRotation` (`SceneComponent.K2_GetComponentLocation` (`self.ProjectileSpawn`)) (`self.K2_GetActorLocation` (`GameplayStatics.GetPlayerCharacter` 0)))))
  (`self.K2_SetActorRelativeRotation` (stale `self.Attack` _sunbeam) (`KismetMathLibrary.MakeRotator` 0.0 _returnvalue_pitch) false false)
  (bind _hit_location (`self.UpdateBeam`))
  (set `/Game/Enemies/BP_Sunbeam.BeamEnd` (+ _hit_location (0.0 0.0 100.0)) (stale `self.Attack` _sunbeam)))

(event `self.Enter Combat`
  ;[1 1 1] Handles entering + exiting combat
  (`PrimitiveComponent.SetMaterial` (`self.AttackIndicator`) 0 "/Game/Enemies/TestStuff/M_TestMaterial_Yellow.M_TestMaterial_Yellow")
  (set `self.InCombat` true)
  (`self.EnterCombat`))

(event `self.Exit Combat`
  ;[1 1 1] Handles entering + exiting combat
  (`PrimitiveComponent.SetMaterial` (`self.AttackIndicator`) 0 "/Game/Enemies/TestStuff/M_TestMaterial_Green.M_TestMaterial_Green")
  (set `self.InCombat` false)
  (`self.ExitCombat`)
  (`self.Reset Rotation`))

(event `self.ChargeAttack`
  ;[1 1 1] Handles enemy attack charging
  (`PrimitiveComponent.SetMaterial` (`self.AttackIndicator`) 0 "/Game/Enemies/TestStuff/M_TestMaterial_Orange.M_TestMaterial_Orange")
  (`KismetSystemLibrary.Delay` (`self.AttackChargeTime`))
  (`self.ChargeComplete`))

(event `Reset Rotation`
  (bind _returnvalue (`self.K2_GetActorRotation`))
  (bind _defaultrotation (`self.DefaultRotation`))
  ;[1 1 1] Resets rotation to default
  (if (not (or (== _returnvalue _defaultrotation) (`self.InCombat`))) :!label _label
    (`self.K2_SetActorRotation` (`KismetMathLibrary.RInterpTo` _returnvalue _defaultrotation (* (`GameplayStatics.GetWorldDeltaSeconds`) 5.0) 0.8))
    (`KismetSystemLibrary.DelayUntilNextTick`)
    (goto _label)))

(event `self.ReceiveBeginPlay`
  ;[1 1 1] Initialises stuff
  (`AIController.RunBehaviorTree` (`AIBlueprintHelperLibrary.GetAIController` self) "/Game/Enemies/Gargoyle/BT_Gargoyle.BT_Gargoyle")
  (set `self.DefaultRotation` (`self.K2_GetActorRotation`))
  (`parent.ReceiveBeginPlay`))

(fn `Shoot`
  (returns (Sunbeam :type "/Game/Enemies/BP_Sunbeam Object Reference"))
  (bind _returnvalue (`SceneComponent.K2_GetComponentLocation` (`self.ProjectileSpawn`)))
  (bind (_returnvalue_roll _returnvalue_pitch) (`KismetMathLibrary.BreakRotator` (`KismetMathLibrary.FindLookAtRotation` _returnvalue (`self.K2_GetActorLocation` (`GameplayStatics.GetPlayerCharacter` 0)))))
  (bind _returnvalue_2 (`|SpawnActorFromClass` "/Game/Enemies/BP_Sunbeam.BP_Sunbeam_C" (`KismetMathLibrary.MakeTransform` _returnvalue (`KismetMathLibrary.MakeRotator` 0.0 _returnvalue_pitch) (0.8 0.8 2.4)) "Undefined" "MultiplyWithRoot" null 0.4 5.0 (+ (`self.K2_GetActorLocation`) (* (`self.GetActorForwardVector`) (`self.BeamRange`))) 10.0 null))
  (`self.K2_AttachToComponent` _returnvalue_2 (`self.ProjectileSpawn`) "None" "SnapToTarget" "KeepRelative" "KeepRelative" true)
  (return _returnvalue_2))

(fn `Spawn Projectiles`
  (params (Shots :type Integer))
  (bind _returnvalue (`SceneComponent.K2_GetComponentLocation` (`self.ProjectileSpawn`)))
  (for _ (range Shots)
    (`|SpawnActorFromClass` "/Game/Enemies/Projectiles/BP_Projectile_Base.BP_Projectile_Base_C" (`KismetMathLibrary.MakeTransform` _returnvalue (`KismetMathLibrary.FindLookAtRotation` _returnvalue (`self.K2_GetActorLocation` (`GameplayStatics.GetPlayerCharacter` 0)))) "Undefined" "MultiplyWithRoot" null 5.0 750.0 null null)))

(fn `UpdateBeam`
  (returns (`Hit Location` :type "Vector Structure"))
  (bind _returnvalue (`self.K2_GetActorLocation`))
  (bind (_returnvalue_x _returnvalue_y) (`KismetMathLibrary.BreakVector` (+ _returnvalue (* (`self.GetActorForwardVector`) (`self.BeamRange`)))))
  (bind _outactors (`GameplayStatics.GetAllActorsOfClass` "/Script/Engine.TriggerVolume"))
  (bind _outhit (`KismetSystemLibrary.LineTraceSingleForObjects` _returnvalue (`KismetMathLibrary.MakeVector` _returnvalue_x _returnvalue_y (`self.Calculate Beam Z Value`)) (`|MakeArray` "ObjectTypeQuery3" "ObjectTypeQuery1" :!type "EObjectTypeQuery Enum") false _outactors))
  (return (`.Location` (`GameplayStatics.BreakHitResult` _outhit))))

(fn `UserConstructionScript`
  (`parent.UserConstructionScript`))