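; Possessed armour enemy that charges at the player and only takes player damage from behind while not attacking.
; An attack plays a montage while a looping timer turns it toward the player, then a notify starts a timer-driven impulse charge.
; Reaching charge distance or hitting the player triggers a sphere-trace melee, with knockback on collision, then a cooldown.
; Combat and attack phases swap indicator materials, and most also adjust walk speed.
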(event `self.Enter Combat`
  ;[1 1 1] Enter/exit Combat
  (`PrimitiveComponent.SetMaterial` (`self.AttackIndicator`) 0 "/Game/Enemies/TestStuff/M_TestMaterial_Yellow.M_TestMaterial_Yellow")
  (set `self.InCombat` true)
  (set `CharacterMovementComponent.MaxWalkSpeed` (`self.AggressiveSpeed`) (`self.CharacterMovement`))
  (`self.EnterCombat`))

(event `self.ReceiveAnyDamage`
  (params (Damage :type "Float (single-precision)") (DamageType :type "DamageType Object Reference") (InstigatedBy :type "Controller Object Reference") (DamageCauser :type "Actor Object Reference"))
  ;[1 1 1] Damage Handling
  (if (== DamageCauser (`GameplayStatics.GetPlayerCharacter` 0))
    (if (and (`self.Check If Player Behind` DamageCauser) (not (`self.IsAttacking`)))
      (`parent.ReceiveAnyDamage` Damage DamageType InstigatedBy DamageCauser :!label _label))
    (else
      (goto _label))))

(event `self.Exit Combat`
  ;[1 1 1] Enter/exit Combat
  (`PrimitiveComponent.SetMaterial` (`self.AttackIndicator`) 0 "/Game/Enemies/TestStuff/M_TestMaterial_Green.M_TestMaterial_Green")
  (set `self.InCombat` false)
  (set `CharacterMovementComponent.MaxWalkSpeed` (`self.PassiveSpeed`) (`self.CharacterMovement`))
  (`self.ExitCombat`))

(event `Rotate`
  ;[1 1 1] Aim at player before charging
  (`self.K2_SetActorRotation` (`self.Calculate Rotation` 5.0)))

(event `NotifyBeginCharge`
  ;[1 0.09 0.09] Begin Attack Process
  (`KismetSystemLibrary.K2_ClearAndInvalidateTimerHandle` (stale `self.Attack` _returnvalue))
  (`PrimitiveComponent.SetMaterial` (`self.AttackIndicator`) 0 "/Game/Enemies/TestStuff/M_TestMaterial_Red.M_TestMaterial_Red")
  (`self.beginCharge`))

(event `self.Attack`
  (bind _asabp_possessed_armour (cast `/Game/Enemies/PossessedArmour/ABP_Possessed_Armour` (`self.AnimationBP`) :!pure true))
  ;[1 0.09 0.09] Begin Attack Process
  (if (`self.CanAttack`)
    (`PrimitiveComponent.SetMaterial` (`self.AttackIndicator`) 0 "/Game/Enemies/TestStuff/M_TestMaterial_Orange.M_TestMaterial_Orange")
    (`self.PlayAnimMontage` "/Game/Enemies/PossessedArmour/Animations/AM_Charge_Montage.AM_Charge_Montage" 0.8 "Default")
    (set `self.IsAttacking` true)
    (bind _returnvalue (`KismetSystemLibrary.K2_SetTimerDelegate` (delegate `Rotate`) 0.05 true))
    (set `/Game/Enemies/PossessedArmour/ABP_Possessed_Armour.IsAttacking` true _asabp_possessed_armour)
    (`/Game/Enemies/PossessedArmour/ABP_Possessed_Armour.BeginChargeAttack` _asabp_possessed_armour)))

(event `self.FinishAttackCycle`
  ;[0.21 1 0.9141] Finish Attack Process
  (`KismetSystemLibrary.Delay` (`self.CooldownTime`))
  (`self.AttackComplete`)
  (`PrimitiveComponent.SetMaterial` (`self.AttackIndicator`) 0 "/Game/Enemies/TestStuff/M_TestMaterial_Yellow.M_TestMaterial_Yellow")
  (set `self.IsAttacking` false))

(event `BeginCharge`
  ;[1 0.4708 0.05] Begin Charging
  (set `self.IsCharging` true)
  (set `CharacterMovementComponent.MaxWalkSpeed` (`self.Charge Speed`) (`self.CharacterMovement`))
  (add `self.TriggerMelee` (delegate `Melee`))
  (set `self.Charge Origin` (`self.K2_GetActorLocation`))
  (bind _returnvalue (`KismetSystemLibrary.K2_SetTimerDelegate` (delegate `Charge`) 0.01 true))
  (set `self.ChargeHandle` _returnvalue))

(event `Charge`
  ;[0.9131 1 0.1144] Charge Mechanic
  (`self.Charge Add Impulse`)
  (if (`self.Check Charge Distance Reached`)
    (`KismetSystemLibrary.K2_ClearAndInvalidateTimerHandle` (`self.ChargeHandle`))
    (`self.TriggerMelee`)))

(event `Melee`
  ;[0.05 1 0.101] Finish Charge, Deal Damage
  (`/Game/Enemies/PossessedArmour/ABP_Possessed_Armour.Swing` (cast `/Game/Enemies/PossessedArmour/ABP_Possessed_Armour` (`self.AnimationBP`) :!pure true))
  (remove `self.TriggerMelee` (delegate `Melee`))
  (set `self.IsCharging` false)
  (set `self.IsAttacking` false)
  (`MovementComponent.StopMovementImmediately` (`self.CharacterMovement`))
  (`KismetSystemLibrary.K2_ClearAndInvalidateTimerHandle` (`self.ChargeHandle`))
  (bind _outhit_hitactor (`self.Attack Trace`))
  (`GameplayStatics.ApplyDamage` _outhit_hitactor (`self.Damage`) null null "/Script/Engine.DamageType")
  (set `CharacterMovementComponent.MaxWalkSpeed` (`self.AggressiveSpeed`) (`self.CharacterMovement`))
  (`self.FinishAttackCycle`))

(event `self.CapsuleComponent.OnComponentHit`
  (params (HitComponent :type "PrimitiveComponent Object Reference") (OtherActor :type "Actor Object Reference") (OtherComp :type "PrimitiveComponent Object Reference") (NormalImpulse :type "Vector Structure") (Hit :type "HitResult Structure (by ref)"))
  ;[0.9131 1 0.1144] Charge Collision Check
  (if (and (== OtherActor (`GameplayStatics.GetPlayerCharacter` 0)) (`self.IsCharging`))
    (`self.Melee`)
    (`self.LaunchCharacter` (`GameplayStatics.GetPlayerCharacter` 0) (* (`self.GetActorForwardVector`) (`self.Charge Knockback`)) false false)))

(event `self.ReceiveBeginPlay`
  (`SceneComponent.K2_AttachToComponent` (`self.Cube`) (`self.Mesh`) "Armour_Chest" "KeepWorld" "KeepWorld" "KeepWorld" true)
  (`parent.ReceiveBeginPlay`))

(fn `Attack Trace`
  (returns (OutHit_HitActor :type "Actor Object Reference"))
  (bind _returnvalue (`self.K2_GetActorLocation`))
  (bind _outhit (`KismetSystemLibrary.SphereTraceSingleForObjects` _returnvalue (+ _returnvalue (* (`self.GetActorForwardVector`) (`self.AttackRange`))) 30.0 (`|MakeArray` "ObjectTypeQuery3" "ObjectTypeQuery1" :!type "EObjectTypeQuery Enum")))
  (return (`.HitActor` (`GameplayStatics.BreakHitResult` _outhit))))

(fn `Charge Add Impulse`
  (`CharacterMovementComponent.AddImpulse` (`self.CharacterMovement`) (* (`self.GetActorForwardVector`) 300.0) true))

(fn `UserConstructionScript`
  (`parent.UserConstructionScript`))