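; BP_Armour_Controller is the AI controller for the Possessed Armour enemy, switching it in and out of combat based on perception of the player.
; It caches the controlled armour pawn on begin play and reacts to AI perception updates for the player character.
; Sensing the player triggers combat, while losing them ends it only if the armour is not attacking and the player is beyond a distance just under the lose-sight radius.
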(event `self.AIPerception.OnTargetPerceptionUpdated`
  (params (Actor :type "Actor Object Reference") (Stimulus :type "AIStimulus Structure"))
  (bind _returnvalue (`GameplayStatics.GetPlayerCharacter` 0))
  (bind _enemy (`self.Enemy`))
  (bind _enemy_2 (`self.Enemy`))
  (if (== Actor _returnvalue)
    (if Stimulus_bSuccessfullySensed
      (if (not (`/Game/Enemies/BP_Enemy_Base.InCombat` _enemy_2))
        (set `/Game/Enemies/BP_Enemy_Base.InCombat` true _enemy_2)
        (`/Game/Enemies/BP_Enemy_Base.Enter Combat` _enemy))
      (elif (not (or (`/Game/Enemies/BP_Enemy_Base.IsAttacking` _enemy_2) (< (`self.GetDistanceTo` _returnvalue) 995.0)))
        (`/Game/Enemies/BP_Enemy_Base.Exit Combat` _enemy)))))

(event `self.ReceiveBeginPlay`
  (set `self.Enemy` (cast `/Game/Enemies/PossessedArmour/BP_Enemy_Possessed_Armour` (`self.K2_GetPawn`) :!pure true)))

(fn `UserConstructionScript`)