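; Thrown boomerang projectile that damages enemies it overlaps and returns to Coco, the player character.
; It first flies along the player's facing direction, with a short looping timer reapplying velocity before it becomes returning and catchable.
; Each tick it spins its mesh and, while returning, turns toward the player at a constant rate to steer its projectile movement.
; Overlapping Coco once catchable restores it to the controller's inventory and destroys it.
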(event `self.ReceiveBeginPlay`
  ;[1 0.4549 0.1176] Sets up the timer for catching the boomerang and it flying straight
  (set `self.Player Facing` (`self.GetActorForwardVector` (`GameplayStatics.GetPlayerCharacter` 0)))
  (`self.Fly`)
  (bind _returnvalue (`KismetSystemLibrary.K2_SetTimerDelegate` (delegate `Fly`) 0.1 true))
  (`KismetSystemLibrary.Delay` 0.2)
  (`KismetSystemLibrary.K2_ClearAndInvalidateTimerHandle` _returnvalue)
  (set `self.Returning` true)
  (set `self.Catchable` true))

(event `Fly`
  ;[1 0.4549 0.1176] Makes the boomerang fly straight for a bit before returning to Coco
  (set `MovementComponent.Velocity` (* (`self.Player Facing`) (`self.FlightSpeed`)) (`self.ProjectileMovement`)))

(event `self.ReceiveTick`
  (params (DeltaSeconds :type "Float (single-precision)"))
  ;[1 0.4549 0.1176] Makes the boomerang fly
  (if (`self.Returning`)
    (`self.K2_SetActorRotation` self (`KismetMathLibrary.RInterpTo_Constant` (`self.K2_GetActorRotation` self) (`KismetMathLibrary.FindLookAtRotation` (`self.K2_GetActorLocation` self) (`self.K2_GetActorLocation` (`GameplayStatics.GetPlayerCharacter` 0))) DeltaSeconds (`self.ReturnSpeed`)) false)
    (set `MovementComponent.Velocity` (* (`self.GetActorForwardVector` self) (`self.FlightSpeed`)) (`self.ProjectileMovement`)))
  ;[1 0.4549 0.1176] Makes boomerang spin
  (`SceneComponent.K2_AddRelativeRotation` (`self.Cube2`) (struct :`Yaw` 10.0) false false))

(event `self.ReceiveActorBeginOverlap`
  (params (OtherActor :type "Actor Object Reference"))
  ;[1 0.4549 0.1176] Checks if the overlap is an enemy or Coco, damages on enemy, destroys on Coco
  (bind _asbp_enemy_base (cast `/Game/Enemies/BP_Enemy_Base` OtherActor)
    (:`then`
      (`GameplayStatics.ApplyDamage` _asbp_enemy_base (`self.BoomerangDamage`) null self "/Script/Engine.DamageType"))
    (:`CastFailed`
      (if (and (== (`GameplayStatics.GetObjectClass` OtherActor) "/Game/CharacterController/BP_Coco.BP_Coco_C") (`self.Catchable`))
        (bind _asbp_coco_controller (cast `/Game/CharacterController/BP_Coco_Controller` (`GameplayStatics.GetPlayerController` 0)))
        (set `/Game/CharacterController/BP_Coco_Controller.BoomerangInInventory` true _asbp_coco_controller)
        (`self.K2_DestroyActor`)))))

(fn `UserConstructionScript`
  (`parent.UserConstructionScript`))