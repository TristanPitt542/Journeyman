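; BP_FragBomb is a timed frag bomb that explodes one second after spawning and damages nearby pawns, sparing the BP_Coco player character.
; On detonation it triggers controller rumble and camera shake, enlarges its sphere and activates a particle effect.
; A multi-sphere trace at the body gathers unique hit actors, applies environmental damage to each, then the bomb destroys itself.
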(event `self.ReceiveBeginPlay`
  (bind _hit_enemies (`self.Hit Enemies`))
  (bind _returnvalue (`SceneComponent.K2_GetComponentLocation` (`self.Body`)))
  ;[1 0.4549 0.1176] On object spawn sets a short timer, after the timer finishes creates a collision bubble and applies damage in a given area then destroys the grenade
  (`KismetSystemLibrary.Delay` 1.0)
  (`PlayerController.K2_ClientPlayForceFeedback` (`GameplayStatics.GetPlayerController` 0) "/Game/Items/ControllerVibrate.ControllerVibrate" "None" false false false)
  (`LegacyCameraShake.StartLegacyCameraShake` (`GameplayStatics.GetPlayerCameraManager` 0) "/Game/CharacterController/BP_BombExplode.BP_BombExplode_C" 1.0 "World")
  (`SceneComponent.SetWorldScale3D` (`self.Sphere`) (5.0 5.0 5.0))
  (`ActorComponent.Activate` (`self.ParticleSystem`) true)
  (bind _asbp_coco (cast `/Game/CharacterController/BP_Coco` (`GameplayStatics.GetPlayerCharacter` 0)))
  (bind _outhits (`KismetSystemLibrary.SphereTraceMultiForObjects` _returnvalue (+ _returnvalue (1.0 1.0 1.0)) (`self.explosion range`) (`|MakeArray` "ObjectTypeQuery3" :!type "EObjectTypeQuery Enum") false (`|MakeArray` _asbp_coco :!type "Actor Object Reference")))
  (for _array_element _outhits
    (bind (_bblockinghit _binitialoverlap _time _distance _location _impactpoint _normal _impactnormal _physmat _hitactor) (`GameplayStatics.BreakHitResult` _array_element))
    (if (not (`KismetArrayLibrary.Array_Contains` _hit_enemies _hitactor))
      (`KismetArrayLibrary.Array_Add` _hit_enemies _hitactor)))
  (for _array_element_2 (`self.Hit Enemies`)
    (`GameplayStatics.ApplyDamage` _array_element_2 (`self.Base Damage`) null self "/Engine/EngineDamageTypes/DmgTypeBP_Environmental.DmgTypeBP_Environmental_C"))
  (`self.K2_DestroyActor`))

(fn `UserConstructionScript`)