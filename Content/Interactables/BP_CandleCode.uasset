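; BP_CandleCode is a candle-order puzzle controller that opens a door when candles are lit in the correct sequence.
; On BeginPlay it hands itself to each candle in its Candles array.
; CandleAdd appends each newly lit candle and compares the active list index by index against the sequence.
; A full match sets Active and calls CheckToOpen on DoorRef; a mismatch extinguishes all active candles after a short delay and clears the list.
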(event `self.ReceiveBeginPlay`
  ;[1 1 1] Sending a Ref of this BP to every Candle in the code sequence
  (for _array_element (`self.Candles`)
    (`/Game/Interactables/BP_Candles.Find The Tie` _array_element self)))

(event `CandleAdd`
  (params (CandleToAdd :type "/Game/Interactables/BP_Candles Object Reference"))
  (bind _activecandles (`self.ActiveCandles`))
  ;[1 1 1] Adding Candles, checking the Sequence, Resetting Candles or Opening the Door
  ;;[1 1 1] Adding a newly activated Candle to an array
  (`KismetArrayLibrary.Array_Append` (`self.ActiveCandles`) (`|MakeArray` CandleToAdd))
  ;;[1 1 1] Comparing the new Candle to the candle in the sequence
  (for (_array_element _array_index) (`self.ActiveCandles`)
    (if (== _array_element (`|GetArrayItem` (`self.Candles`) _array_index))
      ;;[1 1 1] Sending the command to open the Door
      (if (== (`KismetArrayLibrary.Array_Length` (`self.ActiveCandles`)) (`KismetArrayLibrary.Array_Length` (`self.Candles`)))
        (set `self.Active` true)
        (`/Game/Interactables/BP_LockedDoor.CheckToOpen` (`self.DoorRef`)))
      (else
        ;;[1 1 1] Reset and Clear
        (`KismetSystemLibrary.Delay` 0.2)
        (for _array_element_2 _activecandles
          (bind _asbp_candles (cast `/Game/Interactables/BP_Candles` _array_element_2))
          (`/Game/Interactables/BP_Candles.Extinguish` _asbp_candles))
        (`KismetArrayLibrary.Array_Clear` _activecandles)))))

(fn `UserConstructionScript`
  (`parent.UserConstructionScript`))