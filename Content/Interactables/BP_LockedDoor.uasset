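; Locked door interactable that swings open once every Unlocker assigned to it is active.
; On BeginPlay it hands each Unlocker a reference to itself, and CheckToOpen counts the active ones while the door is not open.
; When all are active, a timeline lerps the Arrow component's yaw from its current value toward SwingTarget and CallDoorOpened fires.
; A node to disable door collision is left unconnected.
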(event `self.ReceiveBeginPlay`
  ;[1 1 1] Giving each Unlocker a reference to the door
  (for _array_element (`self.Unlockers`)
    (set `/Game/Interactables/BP_InteractableBase.DoorRef` self _array_element)))

(event `CheckToOpen`
  ;[1 1 1] Checking to see is all Unlockers are active
  (if (not (`self.Open`))
    (set `self.Number Active` 0)
    (for _array_element (`self.Unlockers`)
      (if (`/Game/Interactables/BP_InteractableBase.Active` _array_element)
        (set `self.Number Active` (+ (`self.Number Active`) 1))))
    (if (== (`self.Number Active`) (`KismetArrayLibrary.Array_Length` (`self.Unlockers`)))
      (`self.Open Door`)
      (`self.DoorOpened`))))

(event `Open Door`
  (bind (_relativerotation_roll _relativerotation_pitch _relativerotation_yaw) (`KismetMathLibrary.BreakRotator` (`SceneComponent.RelativeRotation` (`self.Arrow`))))
  ;[1 1 1] Opening the Door
  (bind (_direction _alpha) (`Timeline|OpenDoor` :!via `PlayFromStart`)
    (:`Update`
      (`SceneComponent.K2_SetRelativeRotation` (`self.Arrow`) (`KismetMathLibrary.MakeRotator` 0.0 0.0 (`KismetMathLibrary.Lerp` _relativerotation_yaw (`self.SwingTarget`) _alpha)) false false))))

(fn `UserConstructionScript`)