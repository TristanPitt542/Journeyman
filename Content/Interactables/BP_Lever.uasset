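; BP_Lever is a one-shot interactable lever that notifies a linked door when pulled.
; The first Interact sets Active, then, if DoorRef is valid, calls the door's CheckToOpen and plays the Switch timeline.
; The timeline pitches the Arrow component toward a fixed angle, lerping from its current pitch on each update.
; Without a valid door, the lever still becomes active but does not animate.
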(event `/Game/Interactables/BPI_Interact.Interact`
  (bind _doorref (`self.DoorRef`))
  (bind (_relativerotation_roll _relativerotation_pitch) (`KismetMathLibrary.BreakRotator` (`SceneComponent.RelativeRotation` (`self.Arrow`))))
  (if (not (`self.Active`))
    (set `self.Active` true)
    (`/Engine/EditorBlueprintResources/StandardMacros.IsValid` _doorref
      (:`Is Valid`
        (`/Game/Interactables/BP_LockedDoor.CheckToOpen` _doorref)
        (bind (_direction _alpha) (`Timeline|Switch` :!via `PlayFromStart`)
          (:`Update`
            (`SceneComponent.K2_SetRelativeRotation` (`self.Arrow`) (`KismetMathLibrary.MakeRotator` 0.0 (`KismetMathLibrary.Lerp` _relativerotation_pitch 25.0 _alpha) -90.0) false false)))))))

(fn `UserConstructionScript`
  (`parent.UserConstructionScript`))