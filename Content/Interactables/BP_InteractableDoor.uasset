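; BP_InteractableDoor is an interactable door that swings open once when Interact is called.
; An Active flag blocks repeat interactions and is never reset here.
; A timeline drives the yaw of the Arrow component toward SwingTarget, zeroing its pitch and roll.
; Each update lerps from the current yaw rather than a stored start, so the swing compounds instead of following the Alpha curve directly.
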(event `/Game/Interactables/BPI_Interact.Interact`
  (bind (_relativerotation_roll _relativerotation_pitch _relativerotation_yaw) (`KismetMathLibrary.BreakRotator` (`SceneComponent.RelativeRotation` (`self.Arrow`))))
  (if (not (`self.Active`))
    (set `self.Active` true)
    (bind (_direction _alpha) (`Timeline|Timeline` :!via `PlayFromStart`)
      (:`Update`
        (`SceneComponent.K2_SetRelativeRotation` (`self.Arrow`) (`KismetMathLibrary.MakeRotator` 0.0 0.0 (`KismetMathLibrary.Lerp` _relativerotation_yaw (`self.SwingTarget`) _alpha)) false false)))))

(fn `UserConstructionScript`
  (`parent.UserConstructionScript`))