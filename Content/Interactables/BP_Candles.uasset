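; Interactable candle cluster that lights on interaction and reports to a code holder, apparently as part of a code puzzle.
; FindTheTie stores the code holder reference; Interact on an unlit cluster activates its four fire effects and passes itself to CandleAdd.
; Extinguish clears the lit state and flames, allowing relighting.
; On BeginPlay, CandleNumber sets how many of up to four candles show, with cascading switch branches hiding extras and disabling their collision.
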(event `Find The Tie`
  (params (CodeTie :type "/Game/Interactables/BP_CandleCode Object Reference"))
  ;[1 1 1] Getting a reference to the Code Holder
  (set `self.Code Tie` CodeTie))

(event `Extinguish`
  ;[1 1 1] Putting out the Flame
  (set `self.Active` false)
  (`ActorComponent.SetActive` (`self.Fire1`) false false)
  (`ActorComponent.SetActive` (`self.Fire2`) false false)
  (`ActorComponent.SetActive` (`self.Fire3`) false false)
  (`ActorComponent.SetActive` (`self.Fire4`) false false))

(event `/Game/Interactables/BPI_Interact.Interact`
  ;[1 1 1] Interacting with the Candle
  ;;[1 1 1] Sending a signal off to the Code Holder
  (if (not (`self.Active`))
    (set `self.Active` true)
    (`/Game/Interactables/BP_CandleCode.CandleAdd` (`self.Code Tie`) self)
    ;;[1 1 1] Lighting the Candle visually
    (`ActorComponent.SetActive` (`self.Fire1`) true false)
    (`ActorComponent.SetActive` (`self.Fire2`) true false)
    (`ActorComponent.SetActive` (`self.Fire3`) true false)
    (`ActorComponent.SetActive` (`self.Fire4`) true false)))

(event `self.ReceiveBeginPlay`
  (bind _candle4 (`self.Candle4`))
  (bind _candle3 (`self.Candle3`))
  (bind _candle2 (`self.Candle2`))
  ;[1 1 1] Setting the Ammount of Visible Candles
  (switch `int` (- (`self.Candle Number`) 1)
    (:`0`
      (`SceneComponent.SetVisibility` _candle2 false true)
      (`PrimitiveComponent.SetCollisionEnabled` _candle2 "NoCollision")
      (`SceneComponent.SetVisibility` _candle3 false true :!label _label)
      (`PrimitiveComponent.SetCollisionEnabled` _candle3 "NoCollision"))
    (:`1`
      (goto _label))
    (:`2`
      _))
  (`SceneComponent.SetVisibility` _candle4 false true)
  (`PrimitiveComponent.SetCollisionEnabled` _candle4 "NoCollision"))

(fn `UserConstructionScript`
  (`parent.UserConstructionScript`))