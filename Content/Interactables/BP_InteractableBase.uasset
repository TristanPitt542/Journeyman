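; Base interactable actor that shows a prompt when the BP_Coco character enters its collision box.
; On BeginPlay it places the prompt above the actor's root.
; Box overlaps toggle prompt visibility and disable dashing on BP_Coco_Controller until the character leaves.
; Interact only prints the actor's name; ShowPrompt and HidePrompt are empty, with their one-prompt-at-a-time logic left disconnected.
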(event `/Game/Interactables/BPI_Interact.Interact`
  ;[1 1 1] Simple Test
  (`KismetSystemLibrary.PrintString` (`KismetSystemLibrary.GetDisplayName` self)))

(event `/Game/Interactables/BPI_Interact.Show Prompt`
  ;[1 1 1] Showing the Interaction Prompt (also hiding it when it is used)
)

(event `/Game/Interactables/BPI_Interact.Hide Prompt`
  ;[1 1 1] Hiding the Interact Prompt
)

(event `self.ReceiveBeginPlay`
  ;[1 1 1] Set prompt location
  (`SceneComponent.K2_SetWorldLocation` (`self.Prompt`) (+ (`SceneComponent.K2_GetComponentLocation` (`self.DefaultSceneRoot`)) (0.0 0.0 100.0)) false false))

(event `self.coll box.OnComponentBeginOverlap`
  (params (OverlappedComponent :type "PrimitiveComponent Object Reference") (OtherActor :type "Actor Object Reference") (OtherComp :type "PrimitiveComponent Object Reference") (OtherBodyIndex :type Integer) (bFromSweep :type Boolean) (SweepResult :type "HitResult Structure (by ref)"))
  ;[1 1 1] Set prompt visible
  (if (== (`GameplayStatics.GetObjectClass` OtherActor) "/Game/CharacterController/BP_Coco.BP_Coco_C")
    (`SceneComponent.SetVisibility` (`self.Prompt`) true false)
    (bind _asbp_coco_controller (cast `/Game/CharacterController/BP_Coco_Controller` (`GameplayStatics.GetPlayerController` 0)))
    (set `/Game/CharacterController/BP_Coco_Controller.CanDash` false _asbp_coco_controller)))

(event `self.coll box.OnComponentEndOverlap`
  (params (OverlappedComponent :type "PrimitiveComponent Object Reference") (OtherActor :type "Actor Object Reference") (OtherComp :type "PrimitiveComponent Object Reference") (OtherBodyIndex :type Integer))
  ;[1 1 1] set prompt hidden
  (if (== (`GameplayStatics.GetObjectClass` OtherActor) "/Game/CharacterController/BP_Coco.BP_Coco_C")
    (`SceneComponent.SetVisibility` (`self.Prompt`) false false)
    (bind _asbp_coco_controller (cast `/Game/CharacterController/BP_Coco_Controller` (`GameplayStatics.GetPlayerController` 0)))
    (set `/Game/CharacterController/BP_Coco_Controller.CanDash` true _asbp_coco_controller)))

(fn `UserConstructionScript`)