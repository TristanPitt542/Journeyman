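; BP_BigLockedDoor is a double door that swings open when its OpenDoor event is called.
; On BeginPlay it passes itself to each entry in Unlockers as DoorRef, so those objects can reach the door.
; OpenDoor plays a timeline that yaws two Arrow pivots toward opposite SwingTarget angles, lerping from their current rotation each update.
; An unconnected node for disabling door collision is left as an option.
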(event `self.ReceiveBeginPlay`
  (for _array_element (`self.Unlockers`)
    (set `/Game/Interactables/BP_InteractableBase.DoorRef` self _array_element)))

(event `self.Open Door`
  (bind (_relativerotation_roll _relativerotation_pitch _relativerotation_yaw) (`KismetMathLibrary.BreakRotator` (`SceneComponent.RelativeRotation` (`self.Arrow`))))
  (bind (_relativerotation_roll_2 _relativerotation_pitch_2 _relativerotation_yaw_2) (`KismetMathLibrary.BreakRotator` (`SceneComponent.RelativeRotation` (`self.Arrow1`))))
  ;[1 1 1] Opening the Door
  (bind (_direction _alpha) (`Timeline|Timeline` :!via `PlayFromStart`)
    (:`Update`
      (`SceneComponent.K2_SetRelativeRotation` (`self.Arrow`) (`KismetMathLibrary.MakeRotator` 0.0 0.0 (`KismetMathLibrary.Lerp` _relativerotation_yaw (`self.SwingTarget`) _alpha)) false false)
      (`SceneComponent.K2_SetRelativeRotation` (`self.Arrow1`) (`KismetMathLibrary.MakeRotator` 0.0 0.0 (`KismetMathLibrary.Lerp` _relativerotation_yaw_2 (* (`self.SwingTarget`) -1.0) _alpha)) false false))))

(fn `UserConstructionScript`
  (`parent.UserConstructionScript`))