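; BP_StatueSave is a save-point statue where the player, as BP_Coco, saves progress by interacting.
; Its Interact event gets the save data from the player pawn and passes it to the game instance's SavePlayerMessage as a synchronous save.
; CollBox overlaps with BP_Coco show or hide the prompt and toggle CanDash on the player controller, disabling dash while inside.
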(event `/Game/Interactables/BPI_Interact.Interact`
  ;[1 1 1] Save on overlap (Change this to an interact)
  (bind _asbp_coco (cast `/Game/CharacterController/BP_Coco` (`GameplayStatics.GetPlayerPawn` 0)))
  (bind _playersave (`/Game/CharacterController/BP_Coco.Get Player Save` _asbp_coco))
  (message `/Game/Saves/BPI_SaveGame.SavePlayer` (`GameplayStatics.GetGameInstance`) false _playersave))

(event `self.coll box.OnComponentBeginOverlap`
  (params (OverlappedComponent :type "PrimitiveComponent Object Reference") (OtherActor :type "Actor Object Reference") (OtherComp :type "PrimitiveComponent Object Reference") (OtherBodyIndex :type Integer) (bFromSweep :type Boolean) (SweepResult :type "HitResult Structure (by ref)"))
  ;[1 1 1] Set prompt visible
  (if (== (`GameplayStatics.GetObjectClass` OtherActor) "/Game/CharacterController/BP_Coco.BP_Coco_C")
    (`SceneComponent.SetVisibility` (`self.Prompt`) true false)
    (bind _asbp_coco_controller (cast `/Game/CharacterController/BP_Coco_Controller` (`GameplayStatics.GetPlayerController` 0)))
    (set `/Game/CharacterController/BP_Coco_Controller.CanDash` false _asbp_coco_controller)))

(event `self.coll box.OnComponentEndOverlap`
  (params (OverlappedComponent :type "PrimitiveComponent Object Reference") (OtherActor :type "Actor Object Reference") (OtherComp :type "PrimitiveComponent Object Reference") (OtherBodyIndex :type Integer))
  ;[1 1 1] set prompt hidden
  (if (== (`GameplayStatics.GetObjectClass` OtherActor) "/Game/CharacterController/BP_Coco.BP_Coco_C")
    (`SceneComponent.SetVisibility` (`self.Prompt`) false false)
    (bind _asbp_coco_controller (cast `/Game/CharacterController/BP_Coco_Controller` (`GameplayStatics.GetPlayerController` 0)))
    (set `/Game/CharacterController/BP_Coco_Controller.CanDash` true _asbp_coco_controller)))

(fn `UserConstructionScript`)