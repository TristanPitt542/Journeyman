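; BP_Coco is the player character, with camera-relative movement, stamina-based dash, melee attacks, crossbow, timed powerup and enemy lock-on.
; Sphere traces drive attacks and lock-on; charged hits can drain health from enemies, and reloading spends health on arrows.
; An interface line trace shows interact prompts and disables the controller's dash.
; BeginPlay restores game-instance save data and starts stamina regen; stats update BP_UI, and death opens LVL_Castle.
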(event Custom|Powerup%20Event
  ;[1 1 1] Powerup
  (Utilities|FlowControl|Delay (Variables|Default|GetPowerUpDurration))
  (Variables|/Script/Engine.CharacterMovementComponent|SetMaxWalkSpeed (Variables|Character|GetCharacterMovement) (Variables|Default|GetOriginalSpeed))
  (Variables|Default|SetBaseDamage 5e+01))

(event Custom|Dash%20Delay
  ;[1 1 1] Beginplay
  ;;[1 1 1] Stamina Replenish
  (Variables|Default|SetHasDashed true)
  (Utilities|FlowControl|RetriggerableDelay (Variables|Movement|GetDashCooldown))
  (Variables|Default|SetHasDashed false))

(event Custom|Stamina%20Regen
  ;[1 1 1] Beginplay
  ;;[1 1 1] Stamina Replenish
  (if (Variables|Default|GetShouldRegen)
    (if (< (Variables|Movement|GetStamina) 1e+02)
      (if (not (Variables|Default|GetHasDashed))
        (bind _output_get (Variables|Movement|SetStamina (Math|Float|Clamp(Float) (+ (Variables|Movement|GetStamina) (Variables|Movement|GetStaminaReplenish)) 0.0 1e+02)))
        (Default|SetStamina (Variables|Default|GetUI) _output_get)))))

(event Custom|StartReload
  ;[1 1 1] Reload
  (if (< (Variables|Attributes|GetArrowsLeft) (Variables|Default|GetMaxArrows))
    (Variables|Default|SetCanFireCrossbow false)
    (Utilities|FlowControl|Delay (Variables|Default|GetTimeToReload))
    (CallFunction|ReloadCrossbow)))

(event Custom|Stamina%20Drained
  ;[1 1 1] Called when player stamina drained by sunbeam
  (Utilities|FlowControl|RetriggerableDelay 0.5)
  (Variables|Default|SetShouldRegen true))

(event Custom|CheckInteract
  (bind _returnvalue (Game|GetPlayerController 0))
  ;[1 1 1] Interact
  (bind _outhit (Collision|LineTraceByChannel (Transformation|GetActorLocation) (+ (Transformation|GetActorLocation) (* (Transformation|GetActorForwardVector) (Variables|Default|GetInteraction%20Length))) "TraceTypeQuery1" false 0 "None"))
  (if (.bBlockingHit (Collision|BreakHitResult _outhit))
    (if (Utilities|DoesObjectImplementInterface (.HitActor (Collision|BreakHitResult _outhit)) 0)
      (bind _output_get (Variables|Default|SetInteractActor (.HitActor (Collision|BreakHitResult _outhit))))
      (Class|BPIInteract|ShowPrompt(Message) _output_get)
      (bind _asbp_coco_controller (Utilities|Casting|CastToBP_Coco_Controller _returnvalue))
      (Variables|/Game/CharacterController/BP_Coco_Controller.BP_Coco_Controller_C|SetCanDash _asbp_coco_controller false))
    (else
      (Class|BPIInteract|HidePrompt(Message) _output_get)
      (bind _asbp_coco_controller_2 (Utilities|Casting|CastToBP_Coco_Controller _returnvalue))
      (Variables|/Game/CharacterController/BP_Coco_Controller.BP_Coco_Controller_C|SetCanDash _asbp_coco_controller_2 true))))

(event Game|Damage|EventAnyDamage
  (params (Damage :type Float%20%28single-precision%29) (DamageType :type Damage%20Type%20Object%20Reference) (InstigatedBy :type Controller%20Object%20Reference) (DamageCauser :type Actor%20Object%20Reference))
  ;[1 1 1] Damaged
  (bind _output_get (Variables|Default|SetHealth (- (Variables|Default|GetHealth) Damage)))
  (Game|Feedback|ClientPlayForceFeedback (Game|GetPlayerController 0) "/Game/Items/ControllerVibrate.ControllerVibrate" "None" false false false)
  (Class|LegacyCameraShake|StartLegacyCameraShake (Game|GetPlayerCameraManager 0) "/Game/CharacterController/BP_BombExplode.BP_BombExplode_C" 1.5 "World" "0, 0, 0")
  (Default|SetHealth (Variables|Default|GetUI) _output_get)
  (if (<= (Variables|Default|GetHealth) 0.0)
    (CallFunction|Death)))

(event EventBeginPlay
  ;[1 1 1] Beginplay
  (bind _savegamedata (Class|BPISaveGame|GetGameData(Message) (Game|GetGameInstance)))
  (Utilities|IsValid _savegamedata
    (:Is%20Valid
      (CallFunction|UsePlayerSave (Variables|/Game/Saves/BP_SaveGame.BP_SaveGame_C|GetPlayerSave _savegamedata))
      (Utilities|FlowControl|Sequence
        (:then_0
          (bind _asbp_ui (Utilities|Casting|CastToBP_UI (HUD|GetHUD (Game|GetPlayerController 0))))
          (bind _output_get (Variables|Default|SetUI _asbp_ui))
          ;;[1 1 1] Stamina Replenish
          (Default|UpdateItemCount _output_get (Variables|Attributes|GetHoly%20Water%20Count) (Variables|Attributes|GetGarlic%20Bomb%20Count) (Variables|Attributes|GetArrowsLeft))
          (Utilities|Time|SetTimerbyEvent (delegate Custom|Stamina%20Regen) 0.01 true))
        (:then_1
          (bind _outactors (Actor|GetAllActorsOfClass "/Script/Engine.StaticMeshActor"))
          (Variables|Default|SetStaticMeshes _outactors))))
    (:Is%20Not%20Valid
      (Development|PrintString "Error when getting game data"))))

(event Input|KeyboardEvents|DebugKeyT
  (params (Key :type Key%20Structure :default "None") (ActionValue :type Input%20Action%20Value%20Structure))
  (:Pressed
    (bind _result (Math|Integer|IncrementInt (Variables|Attributes|GetGarlic%20Bomb%20Count))
      (:%20%20
        (bind _result_2 (Math|Integer|IncrementInt (Variables|Attributes|GetHoly%20Water%20Count))
          (:%20%20
            (Default|UpdateItemCount (Variables|Default|GetUI) _result_2 _result -1)))))))

(fn ConstructionScript)

(fn Movement
  (params (X%20Value :type Float%20%28double-precision%29) (Y%20Value :type Float%20%28double-precision%29))
  (bind _camera (Variables|Default|GetCamera))
  (bind _returnvalue (Transformation|GetWorldRotation _camera))
  ;[1 1 1] Reads player input and sets for next ticks
  (if (Variables|Default|GetCanMove)
    (Pawn|Input|AddMovementInput (Math|Vector|GetRightVector (Math|Rotator|MakeRotator (.roll _returnvalue) 0.0 (.yaw _returnvalue))) X%20Value false)
    (Pawn|Input|AddMovementInput (Math|Vector|GetForwardVector (Math|Rotator|MakeRotator 0.0 0.0 (.yaw (Transformation|GetWorldRotation (Variables|Default|GetCamera))))) Y%20Value false)))

(fn Dash
  (params (Dash%20Multiplier :type Float%20%28double-precision%29) (X :type Float%20%28double-precision%29) (Y :type Float%20%28double-precision%29))
  (bind _returnvalue (Transformation|GetActorForwardVector))
  (bind _dashdistance (Variables|Movement|GetDashDistance))
  (bind _camera (Variables|Default|GetCamera))
  (bind _returnvalue_2 (Transformation|GetWorldRotation _camera))
  (bind _returnvalue_3 (* Dash%20Multiplier _dashdistance))
  (bind _returnvalue_4 (* _returnvalue _returnvalue_3))
  ;[1 1 1] Dash Mechanics
  (if (<= (Variables|Movement|GetStamina) 0.0)
    (Animation|StopAnimMontage "/Game/CharacterController/Animations/AM_Coco_Dodge.AM_Coco_Dodge")
    (else
      (Transformation|SetActorRotation (Math|Conversions|RotationFromXVector (Math|Vector|RotateVector (Math|Vector|MakeVector X Y 0.0) (Math|Rotator|MakeRotator (.roll _returnvalue_2) 0.0 (.yaw _returnvalue_2)))))
      (Variables|/Script/Engine.MovementComponent|SetVelocity (Variables|Character|GetCharacterMovement) (Math|Vector|MakeVector (.x _returnvalue_4) (.y _returnvalue_4) (.z (Variables|/Script/Engine.MovementComponent|GetVelocity (Variables|Character|GetCharacterMovement)))))
      (bind _output_get (Variables|Movement|SetStamina (- (Variables|Movement|GetStamina) 1.5)))
      (CallFunction|DashDelay)
      (Default|SetStamina (Variables|Default|GetUI) _output_get))))

(fn BasicAttack
  (bind _capsulecomponent (Variables|Collision|GetCapsuleComponent))
  (bind _hitenemies (Variables|Default|GetHitEnemies))
  (bind _returnvalue (Transformation|GetWorldLocation _capsulecomponent))
  ;[1 1 1] charge attack
  (if (Variables|Default|GetCanAttack)
    (Variables|Default|SetCanAttack false)
    (Variables|/Script/Engine.CharacterMovementComponent|SetMaxWalkSpeed (Variables|Character|GetCharacterMovement) 2e+02)
    (bind _outhits (Collision|MultiSphereTraceForObjects _returnvalue (+ _returnvalue (* (Math|Vector|GetForwardVector _capsulecomponent) 1.5e+02)) (Variables|Default|GetBasicAttackRange) (Utilities|Array|MakeArray "ObjectTypeQuery3") false 0 "None" true "(R=1.000000,G=0.824260,B=0.000000,A=1.000000)"))
    (for _array_element _outhits
      (if (not (Utilities|Array|ContainsItem _hitenemies (.HitActor (Collision|BreakHitResult _array_element))))
        (Utilities|Array|Add _hitenemies (.HitActor (Collision|BreakHitResult _array_element)))))
    (for _array_element_2 _hitenemies
      (Game|Damage|ApplyDamage _array_element_2 (Variables|Default|GetBaseDamage) 0 self "/Script/Engine.DamageType")
      (Utilities|Array|Clear _hitenemies))))

(fn ChargeAttack
  (bind _hitenemies (Variables|Default|GetHitEnemies))
  (bind _capsulecomponent (Variables|Collision|GetCapsuleComponent))
  (bind _returnvalue (Transformation|GetWorldLocation _capsulecomponent))
  ;[1 1 1] charge attack
  (if (Variables|Default|GetCanAttack)
    (Variables|Default|SetCanAttack false)
    (Variables|Default|SetCanMove false)
    (bind _outhits (Collision|MultiSphereTraceForObjects _returnvalue (+ _returnvalue (* (Math|Vector|GetForwardVector _capsulecomponent) 1.5e+02)) (Variables|Default|GetBasicAttackRange) (Utilities|Array|MakeArray "ObjectTypeQuery3" "ObjectTypeQuery2") false 0 "None" true "(R=1.000000,G=0.000000,B=0.693892,A=1.000000)"))
    (for _array_element _outhits
      (if (not (Utilities|Array|ContainsItem _hitenemies (.HitActor (Collision|BreakHitResult _array_element))))
        (Utilities|Array|Add _hitenemies (.HitActor (Collision|BreakHitResult _array_element)))))
    (for _array_element_2 _hitenemies
      (Game|Damage|ApplyDamage _array_element_2 (* (Variables|Default|GetBaseDamage) 2.5) 0 self "/Game/CocoChargedAttack.CocoChargedAttack_C")
      (if (.bSuccess (Utilities|Casting|CastToBP_Enemy_Base (.HitActor (Collision|BreakHitResult _array_element))))
        (bind _output_get (Variables|Default|SetHealth (Math|Float|Clamp(Float) (+ (Variables|Default|GetHealth) (Variables|Default|GetDrainHealth)) 0.0 1e+02)))
        (Default|ChangeHealth (Variables|Default|GetUI) _output_get)))
    (Utilities|Array|Clear (Variables|Default|GetHitEnemies))))

(fn Powerup
  ;[1 1 1] Powerup
  (Variables|/Script/Engine.CharacterMovementComponent|SetMaxWalkSpeed (Variables|Character|GetCharacterMovement) (Variables|Default|GetPowerupSpeed))
  (Variables|Default|SetBaseDamage (* (Variables|Default|GetBaseDamage) 2.0)))

(fn Death
  (Game|OpenLevel(byName) "LVL_Castle"))

(fn EngageLockon
  (params (Actors%20to%20Ignore :type Array%20of%20Actor%20Object%20References))
  (bind _capsulecomponent (Variables|Collision|GetCapsuleComponent))
  (bind _returnvalue (Transformation|GetWorldLocation _capsulecomponent))
  (bind (_outhits _returnvalue_2) (Collision|MultiSphereTraceForObjects _returnvalue (+ _returnvalue 1) (Variables|Default|GetLockOnRadius) (Utilities|Array|MakeArray "ObjectTypeQuery3") false Actors%20to%20Ignore "None"))
  (for _array_element _outhits
    (if _returnvalue_2
      (if (not (Utilities|Array|ContainsItem (Variables|Default|GetNearEnemies) (.HitActor (Collision|BreakHitResult _array_element))))
        (Utilities|Array|Add (Variables|Default|GetNearEnemies) (.HitActor (Collision|BreakHitResult _array_element))))))
  (Variables|Default|SetLockedOn true)
  (bind _output_get (Variables|Default|SetLockedEnemy (.ReturnValue (Actor|FindNearestActor (Transformation|GetWorldLocation (Variables|Collision|GetCapsuleComponent)) (Variables|Default|GetNearEnemies)))))
  (bind _asbp_enemy_base (Utilities|Casting|CastToBP_Enemy_Base _output_get))
  (Default|ShowCircle _asbp_enemy_base)
  (Default|HidePrompt _asbp_enemy_base))

(fn DisengageLockon
  (Variables|Default|SetLockedOn false)
  (Utilities|Array|Clear (Variables|Default|GetNearEnemies))
  (bind _asbp_enemy_base (Utilities|Casting|CastToBP_Enemy_Base (Variables|Default|GetLockedEnemy)))
  (Default|HideCircle _asbp_enemy_base))

(fn FIreArrow
  ;[1 1 1] Spawn arrow
  (if (and (> (Variables|Attributes|GetArrowsLeft) 0) (Variables|Default|GetCanFireCrossbow))
    (Game|SpawnActorfromClass "/Game/Items/BP_Arrow.BP_Arrow_C" (Transformation|GetWorldTransform (Variables|Default|GetProjectile%20Spawn)) "AlwaysSpawn" "MultiplyWithRoot" 0 0)
    (bind _result (Math|Integer|DecrementInt (Variables|Attributes|GetArrowsLeft))
      (:%20%20
        (Default|UpdateItemCount (Variables|Default|GetUI) -1 -1 _result)))))

(fn InvincibilityCheck
  (bind _stamina (Variables|Movement|GetStamina))
  (bind _returnvalue (>= _stamina 3e+01))
  (if _returnvalue
    (Variables|Default|SetInvincible _returnvalue)
    (return _returnvalue)))

(fn ChangeStamina
  (params (Change :type Float%20%28double-precision%29))
  (Variables|Movement|SetStamina (Math|Float|Clamp(Float) (+ (Variables|Movement|GetStamina) Change) 0.0 1e+02))
  (Default|ChangeStamina (Variables|Default|GetUI) Change))

(fn Interaction
  ;[1 1 1] Interaction
  ;;[1 1 1] Making sure the Player can interact
  (bind _outhit (Collision|SphereTraceByChannel (Transformation|GetActorLocation) (+ (Transformation|GetActorLocation) (* (Transformation|GetActorForwardVector) (Variables|Default|GetInteraction%20Length))) 6e+01 "TraceTypeQuery1" false (Variables|Default|GetStaticMeshes) "None"))
  (if true
    (Class|BPIInteract|Interact(Message) (.HitActor (Collision|BreakHitResult _outhit)))))

(fn ReloadCrossbow
  (Utilities|FlowControl|ForLoopwithBreak (Variables|Attributes|GetArrowsLeft) (- (Variables|Default|GetMaxArrows) 1) :!label _label
    (:LoopBody
      (if (>= (- (Variables|Default|GetHealth) (* (+ (Variables|Default|GetArrowsToAdd) 1) (Variables|Default|GetArrowHealthCost))) 15.0)
        (Variables|Default|SetArrowsToAdd (+ (Variables|Default|GetArrowsToAdd) 1))
        (else
          (goto _label Break))))
    (:Completed
      (Variables|Default|SetHealth (- (Variables|Default|GetHealth) (* (Variables|Default|GetArrowsToAdd) (Variables|Default|GetArrowHealthCost))))
      (Variables|Attributes|SetArrowsLeft (+ (Variables|Attributes|GetArrowsLeft) (Variables|Default|GetArrowsToAdd)))
      (Default|ChangeHealth (Variables|Default|GetUI) (Variables|Default|GetHealth))
      (Variables|Default|SetCanFireCrossbow true)
      (Variables|Default|SetArrowsToAdd 0))))

(fn GetPlayerSave
  ;[1 1 1] Get Player Save
  (return (Utilities|Struct|MakeST_SaveGame (Transformation|GetActorTransform) 1e+02 1e+02 (Variables|Attributes|GetArrowsLeft) (Variables|Default|GetMoney) (Variables|Attributes|GetHoly%20Water%20Count) (Variables|Attributes|GetGarlic%20Bomb%20Count) (Variables|Attributes|GetHas%20Boomerang))))

(fn UsePlayerSave
  (params (PlayerSave :type ST%20Save%20Game%20Structure))
  ;[1 1 1] Use Player Save (to use the save after loading back in)
  (if (not (== (.playertransform PlayerSave) (Math|Transform|MakeTransform "0, 0, 0"))) ; Check transform
    (Transformation|SetActorTransform (.playertransform PlayerSave))
    (if (not (== (.playerhealth PlayerSave) 0.0))
      (Variables|Default|SetHealth 1e+02)
      (Utilities|FlowControl|Sequence
        (:then_0
          (if (!= (.playerstamina PlayerSave) 0.0)
            (Variables|Movement|SetStamina 1e+02)))
        (:then_1
          (if (!= (.playerarrows PlayerSave) 0)
            (Variables|Attributes|SetArrowsLeft (.playerarrows PlayerSave))))
        (:then_2
          (if (!= (.coins PlayerSave) 0)
            (Variables|Default|SetMoney (.coins PlayerSave))))
        (:then_3
          (if (!= (.holywatercount PlayerSave) 0)
            (Variables|Attributes|SetHoly%20Water%20Count (.holywatercount PlayerSave))))
        (:then_4
          (if (!= (.garlicbombcount PlayerSave) 0)
            (Variables|Attributes|SetGarlic%20Bomb%20Count (.garlicbombcount PlayerSave))))
        (:then_5
          (if (.hasboomerang PlayerSave)
            (Variables|Attributes|SetHas%20Boomerang (.hasboomerang PlayerSave))))))))

(fn ClosestEnemy
  (bind _capsulecomponent (Variables|Collision|GetCapsuleComponent))
  (bind _returnvalue (Transformation|GetWorldLocation _capsulecomponent))
  (bind (_outhits _returnvalue_2) (Collision|MultiSphereTraceForObjects _returnvalue (+ _returnvalue 1) (Variables|Default|GetLockOnRadius) (Utilities|Array|MakeArray "ObjectTypeQuery3") false 0 "None"))
  (if _returnvalue_2
    (for _array_element _outhits
      (if (not (Utilities|Array|ContainsItem (Variables|Default|GetNearEnemies) (.HitActor (Collision|BreakHitResult _array_element))))
        (Utilities|Array|Add (Variables|Default|GetNearEnemies) (.HitActor (Collision|BreakHitResult _array_element)))))
    (if (not (Variables|Default|GetLockedOn))
      (for _array_element_2 (Variables|Default|GetNearEnemies)
        (bind _asbp_enemy_base (Utilities|Casting|CastToBP_Enemy_Base _array_element_2))
        (Default|HidePrompt _asbp_enemy_base))
      (bind _asbp_enemy_base_2 (Utilities|Casting|CastToBP_Enemy_Base (.ReturnValue (Actor|FindNearestActor (Transformation|GetWorldLocation (Variables|Collision|GetCapsuleComponent)) (Variables|Default|GetNearEnemies)))))
      (Default|ShowPrompt _asbp_enemy_base_2))))