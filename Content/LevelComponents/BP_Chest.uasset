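; BP_Chest is an interactable chest that opens once and ejects an item.
; Interact calls Open, where a timeline pitches the lid, then sets IsOpen and spawns the Item class at the spline's first point.
; A second timeline, rate-scaled by TimeToComplete, moves the item along the spline and sets its CanPickup flag on arrival.
; IsOpen is set only when the lid finishes, so interacting mid-animation restarts the opening.
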(event `/Game/Interactables/BPI_Interact.Interact`
  (if (not (`self.IsOpen`))
    (`self.Open`)))

(event `Open`
  (bind (_relativerotation_roll _relativerotation_pitch _relativerotation_yaw) (`KismetMathLibrary.BreakRotator` (`SceneComponent.RelativeRotation` (`self.Lid`))))
  (bind (_direction _alpha) (`Timeline|OpenChest` :!via `PlayFromStart`)
    (:`Update`
      (`SceneComponent.K2_SetRelativeRotation` (`self.Lid`) (`KismetMathLibrary.MakeRotator` _relativerotation_roll _alpha _relativerotation_yaw) false false))
    (:`Finished`
      (set `self.IsOpen` true)
      (`self.SpawnItem`))))

(event `SpawnItem`
  (bind _returnvalue (`|SpawnActorFromClass` (`self.Item`) (`SplineComponent.GetTransformAtSplinePoint` (`self.Spline`) 0 "World" false) "AlwaysSpawn" "MultiplyWithRoot" null false null))
  (`TimelineComponent.SetPlayRate` (`self.Alpha`) (/ 1.0 (`self.TimeToComplete`)))
  (bind (_direction _alpha) (`Timeline|Alpha`)
    (:`Update`
      (`self.K2_SetActorTransform` _returnvalue (`KismetMathLibrary.MakeTransform` (`SplineComponent.GetLocationAtDistanceAlongSpline` (`self.Spline`) (`KismetMathLibrary.Lerp` 0.0 (`SplineComponent.GetSplineLength` (`self.Spline`)) _alpha) "World")) false false))
    (:`Finished`
      (set `/Game/Pickup/BP_Item_base.CanPickup` true _returnvalue))))

(fn `UserConstructionScript`)