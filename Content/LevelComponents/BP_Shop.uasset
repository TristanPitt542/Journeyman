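; BP_Shop is a level shop actor that spawns four priced pickups at its Item1 to Item4 points on BeginPlay.
; It pairs the ShopItems and Prices arrays by index, stores the pickups and fills each one's WBP_ShopItem widget with name and price.
; Purchasing is absent: Interact is empty, the ShopZone overlap only casts to BP_Coco, and a disconnected loop prints the overlapped pickup's name.
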(event `self.ReceiveBeginPlay`
  (for (_array_element _array_index) (`|MakeArray` (`self.Item 1`) (`self.Item 2`) (`self.Item 3`) (`self.Item 4`))
    (bind _returnvalue_location (`KismetMathLibrary.BreakTransform` (`SceneComponent.K2_GetComponentToWorld` _array_element)))
    (bind _returnvalue (`|SpawnActorFromClass` (`|GetArrayItem` (`self.ShopItems`) _array_index) (`KismetMathLibrary.MakeTransform` _returnvalue_location) "AlwaysSpawn" "MultiplyWithRoot" null (`|GetArrayItem` (`self.Prices`) _array_index) null))
    (`KismetArrayLibrary.Array_Add` (`self.ShopPickups`) _returnvalue)
    (bind _aswbp_shop_item (cast `/Game/UI/Widgets/WBP_ShopItem` (`WidgetComponent.GetWidget` (`/Game/Pickup/Shop/BP_Shop_Item.Widget` _returnvalue))))
    (set `/Game/UI/Widgets/WBP_ShopItem.Name` (`/Game/Pickup/Shop/BP_Shop_Item.Name` _returnvalue) _aswbp_shop_item)
    (set `/Game/UI/Widgets/WBP_ShopItem.Price` (`KismetTextLibrary.Conv_StringToText` (`KismetStringLibrary.Concat_StrStr` "Price : $" (`KismetStringLibrary.Conv_IntToString` (`/Game/Pickup/Shop/BP_Shop_Item.Price` _returnvalue)))) _aswbp_shop_item)))

(event `/Game/Interactables/BPI_Interact.Interact`)

(event `self.ShopZone.OnComponentBeginOverlap`
  (params (OverlappedComponent :type "PrimitiveComponent Object Reference") (OtherActor :type "Actor Object Reference") (OtherComp :type "PrimitiveComponent Object Reference") (OtherBodyIndex :type Integer) (bFromSweep :type Boolean) (SweepResult :type "HitResult Structure (by ref)"))
  (cast `/Game/CharacterController/BP_Coco` OtherActor))

(fn `UserConstructionScript`)