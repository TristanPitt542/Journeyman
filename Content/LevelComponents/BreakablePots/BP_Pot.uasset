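; Breakable pot that releases an item when damaged by BP_Coco, with its mesh chosen from eight variants by Size in the construction script.
; On that damage it hides the mesh and spawns the Item class at the start of its spline.
; A timeline moves the item along the spline, then makes it pickable and destroys the pot.
; Dust and sound effect nodes are present but never run.
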(event `self.ReceiveAnyDamage`
  (params (Damage :type "Float (single-precision)") (DamageType :type "DamageType Object Reference") (InstigatedBy :type "Controller Object Reference") (DamageCauser :type "Actor Object Reference"))
  (if (== (`GameplayStatics.GetObjectClass` DamageCauser) "/Game/CharacterController/BP_Coco.BP_Coco_C")
    (`SceneComponent.SetVisibility` (`self.pot`) false false)
    (bind _returnvalue (`|SpawnActorFromClass` (`self.Item`) (`SplineComponent.GetTransformAtSplinePoint` (`self.Spline`) 0 "World" false) "AlwaysSpawn" "MultiplyWithRoot" null false null))
    (`TimelineComponent.SetPlayRate` (`self.Alpha`) (/ 1.0 (`self.TimeToComplete`)))
    (bind (_direction _alpha) (`Timeline|Timeline`)
      (:`Update`
        (`self.K2_SetActorTransform` _returnvalue (`KismetMathLibrary.MakeTransform` (`SplineComponent.GetLocationAtDistanceAlongSpline` (`self.Spline`) (`KismetMathLibrary.Lerp` 0.0 (`SplineComponent.GetSplineLength` (`self.Spline`)) _alpha) "World")) false false))
      (:`Finished`
        (set `/Game/Pickup/BP_Item_base.CanPickup` true _returnvalue)
        (`self.K2_DestroyActor`)))))

(fn `UserConstructionScript`
  (bind _size (`self.Size`))
  (if (== _size 1)
    (`StaticMeshComponent.SetStaticMesh` (`self.pot`) "/Game/LevelPrototyping/Asset_Kit/Prop_Assets/Pots/SM_Pot_1/SM_Pot_1.SM_Pot_1")
    (elif (== _size 2)
      (`StaticMeshComponent.SetStaticMesh` (`self.pot`) "/Game/LevelPrototyping/Asset_Kit/Prop_Assets/Pots/SM_Pot_2/SM_Pot_2.SM_Pot_2")
      (elif (== _size 3)
        (`StaticMeshComponent.SetStaticMesh` (`self.pot`) "/Game/LevelPrototyping/Asset_Kit/Prop_Assets/Pots/SM_Pot_3/SM_Pot_3.SM_Pot_3")
        (elif (== _size 4)
          (`StaticMeshComponent.SetStaticMesh` (`self.pot`) "/Game/LevelPrototyping/Asset_Kit/Prop_Assets/Pots/SM_Pot_4/SM_Pot_4.SM_Pot_4")
          (elif (== _size 5)
            (`StaticMeshComponent.SetStaticMesh` (`self.pot`) "/Game/LevelPrototyping/Asset_Kit/Prop_Assets/Pots/SM_Pot_5/SM_Pot_5.SM_Pot_5")
            (elif (== _size 6)
              (`StaticMeshComponent.SetStaticMesh` (`self.pot`) "/Game/LevelPrototyping/Asset_Kit/Prop_Assets/Pots/SM_Pot_6/SM_Pot_6.SM_Pot_6")
              (elif (== _size 7)
                (`StaticMeshComponent.SetStaticMesh` (`self.pot`) "/Game/LevelPrototyping/Asset_Kit/Prop_Assets/Pots/SM_Pot_7/SM_Pot_7.SM_Pot_7")
                (elif (== _size 8)
                  (`StaticMeshComponent.SetStaticMesh` (`self.pot`) "/Game/LevelPrototyping/Asset_Kit/Prop_Assets/Pots/SM_Pot_8/SM_Pot_8.SM_Pot_8"))))))))))