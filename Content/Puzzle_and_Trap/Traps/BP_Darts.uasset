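; Dart trap that fires when a pawn overlaps its trigger Box and damages any pawn the darts touch.
; After a delay, a timeline moves the Darts component cumulatively along its right vector, then resets it to the start point saved at BeginPlay.
; A cooldown flag blocks retriggering and clears after a delay started from timeline updates.
; The flag is set before the pawn check, so a non-pawn overlap leaves it set.
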(event `self.ReceiveBeginPlay`
  ;[1 1 1] Set orogin location for dats
  (set `self.darts_start_point` (`SceneComponent.K2_GetComponentLocation` (`self.darts`))))

(event `self.Box.OnComponentBeginOverlap`
  (params (OverlappedComponent :type "PrimitiveComponent Object Reference") (OtherActor :type "Actor Object Reference") (OtherComp :type "PrimitiveComponent Object Reference") (OtherBodyIndex :type Integer) (bFromSweep :type Boolean) (SweepResult :type "HitResult Structure (by ref)"))
  (bind _darts (`self.darts`))
  ;[1 1 1] Shoot Darts
  (if (not (`self.On_cooldown`))
    (set `self.On_cooldown` true)
    (cast `Pawn` OtherActor)
    (`KismetSystemLibrary.Delay` (`self.Duration`))
    (bind (_direction _distance_over_time) (`Timeline|Timeline` :!via `PlayFromStart`)
      (:`Update`
        (`SceneComponent.K2_SetWorldLocation` (`self.darts`) (+ (* _distance_over_time (`SceneComponent.GetRightVector` _darts)) (`SceneComponent.K2_GetComponentLocation` _darts)) false false)
        (`KismetSystemLibrary.Delay` (`self.cooldown`))
        (set `self.On_cooldown` false))
      (:`Finished`
        ;;[1 1 1] Reset location of darts to origin
        (`SceneComponent.K2_SetWorldLocation` (`self.darts`) (`self.darts_start_point`) false false)))))

(event `self.darts.OnComponentBeginOverlap`
  (params (OverlappedComponent :type "PrimitiveComponent Object Reference") (OtherActor :type "Actor Object Reference") (OtherComp :type "PrimitiveComponent Object Reference") (OtherBodyIndex :type Integer) (bFromSweep :type Boolean) (SweepResult :type "HitResult Structure (by ref)"))
  ;[1 1 1] Apply damage
  (bind _aspawn (cast `Pawn` OtherActor))
  (`GameplayStatics.ApplyDamage` _aspawn 10.0 null null "/Script/Engine.DamageType"))

(fn `UserConstructionScript`)