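; BP_Spikes is a trap that moves its spikes when BP_Coco enters its box, damaging the character.
; After a short delay, the Move_up timeline shifts the spikes by per-update offsets, with a delayed overlap check before applying damage.
; On finish it pauses, runs Move_down to rewind, then clears the cooldown after a delay.
; The cooldown flag is set before the cast, so any overlapping actor sets it.
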(event `self.Box.OnComponentBeginOverlap`
  (params (OverlappedComponent :type "PrimitiveComponent Object Reference") (OtherActor :type "Actor Object Reference") (OtherComp :type "PrimitiveComponent Object Reference") (OtherBodyIndex :type Integer) (bFromSweep :type Boolean) (SweepResult :type "HitResult Structure (by ref)"))
  (bind _spikes (`self.spikes`))
  (bind _spikes_2 (`self.spikes`))
  (if (not (`self.On_cooldown`))
    (set `self.On_cooldown` true)
    (bind _asbp_coco (cast `/Game/CharacterController/BP_Coco` OtherActor))
    ;[1 1 1] Activate
    (`KismetSystemLibrary.Delay` 0.2)
    (bind (_direction _newtrack_0) (`Timeline|move_up` :!via `PlayFromStart`)
      (:`Update`
        (`SceneComponent.K2_SetWorldLocation` _spikes (- (`SceneComponent.K2_GetComponentLocation` _spikes) _newtrack_0) false false)
        ;[1 1 1] Apply damage
        (`KismetSystemLibrary.Delay` 0.5)
        (if (`PrimitiveComponent.IsOverlappingActor` (`self.Box`) _asbp_coco)
          (`GameplayStatics.ApplyDamage` _asbp_coco 10.0 null null "/Script/Engine.DamageType")))
      (:`Finished`
        ;[1 1 1] Rewind
        (`KismetSystemLibrary.Delay` 1.0)
        (bind (_direction_2 _newtrack_0_2) (`Timeline|move_down` :!via `PlayFromStart`)
          (:`Update`
            (`SceneComponent.K2_SetWorldLocation` _spikes_2 (- (`SceneComponent.K2_GetComponentLocation` _spikes_2) _newtrack_0_2) false false)
            (`KismetSystemLibrary.Delay` (`self.cooldown`))
            (set `self.On_cooldown` false)))))))

(fn `UserConstructionScript`)