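; BP_Laser_Start is the emitter of a laser puzzle, projecting a beam that powers laser cubes and triggers levers.
; Each Tick it line-traces forward from its Arrow on the Visibility channel and feeds the hit location to the Laser effect's Beam End.
; A hit BP_Laser_Cube becomes the tracked CurrentCrystal and is activated, with the previous one switched off.
; A hit lever receives Activation, while any other result deactivates the tracked cube.
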(event `self.ReceiveTick`
  (params (DeltaSeconds :type "Float (single-precision)"))
  (bind _currentcrystal (`self.CurrentCrystal`))
  (bind _arrow (`self.Arrow`))
  (bind _returnvalue (`SceneComponent.K2_GetComponentLocation` _arrow))
  ;[1 1 1] Laser Projection System
  (bind _outhit (`KismetSystemLibrary.LineTraceSingle` _returnvalue (+ (* (`SceneComponent.GetForwardVector` _arrow) (10000.0 10000.0 10000.0)) _returnvalue) "TraceTypeQuery1"))
  (`NiagaraComponent.SetVariableVec3` (`self.Laser`) "Beam End" (`.Location` (`GameplayStatics.BreakHitResult` _outhit)))
  (bind _asbp_laser_cube (cast `/Game/Puzzle_and_Trap/PuzzleParts/Laser_Puzzles/BP_Laser_Cube` (`.HitActor` (`GameplayStatics.BreakHitResult` _outhit)))
    (:`then`
      (`/Engine/EditorBlueprintResources/StandardMacros.IsValid` _currentcrystal
        (:`Is Valid`
          (if (== _asbp_laser_cube _currentcrystal)
            (if (not (`/Game/Puzzle_and_Trap/PuzzleParts/Laser_Puzzles/BP_Laser_Cube.Active` _asbp_laser_cube))
              (set `self.CurrentCrystal` _asbp_laser_cube :!label _label)
              (set `/Game/Puzzle_and_Trap/PuzzleParts/Laser_Puzzles/BP_Laser_Cube.Active` true _asbp_laser_cube))
            (elif (not (`/Game/Puzzle_and_Trap/PuzzleParts/Laser_Puzzles/BP_Laser_Cube.Active` _asbp_laser_cube))
              (set `/Game/Puzzle_and_Trap/PuzzleParts/Laser_Puzzles/BP_Laser_Cube.Active` false _currentcrystal)
              (set `self.CurrentCrystal` _asbp_laser_cube))))
        (:`Is Not Valid`
          (goto _label))))
    (:`CastFailed`
      (bind _asbp_laser_lever (cast `/Game/Puzzle_and_Trap/PuzzleParts/BP_Laser_Lever` (`.HitActor` (`GameplayStatics.BreakHitResult` _outhit)))
        (:`then`
          (`/Game/Puzzle_and_Trap/PuzzleParts/BP_Laser_Lever.Activation` _asbp_laser_lever))
        (:`CastFailed`
          (`/Engine/EditorBlueprintResources/StandardMacros.IsValid` _currentcrystal
            (:`Is Valid`
              (set `/Game/Puzzle_and_Trap/PuzzleParts/Laser_Puzzles/BP_Laser_Cube.Active` false _currentcrystal))))))))

(fn `UserConstructionScript`)