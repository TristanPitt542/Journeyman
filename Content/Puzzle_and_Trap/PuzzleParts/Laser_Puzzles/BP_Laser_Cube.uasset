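; BP_Laser_Cube is a laser puzzle piece that switches its beam on or off according to its Active flag.
; Every Tick applies the active or inactive material to the Cone and sets the Laser component to match.
; Parent Tick logic runs only while active.
; When inactive, it deactivates any valid CurrentCrystal and resets that reference to NoCrystal.
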(event `self.ReceiveTick`
  (params (DeltaSeconds :type "Float (single-precision)"))
  (bind _currentcrystal (`self.CurrentCrystal`))
  (bind _cone (`self.Cone`))
  ;[1 1 1] Laser Activation
  (if (`self.Active`)
    (`PrimitiveComponent.SetMaterial` _cone 0 (`self.Active Mat`))
    (`ActorComponent.SetActive` (`self.Laser`) true false)
    (`parent.ReceiveTick` DeltaSeconds)
    (else
      (`PrimitiveComponent.SetMaterial` _cone 0 (`self.Inactive Mat`))
      (`ActorComponent.SetActive` (`self.Laser`) false false)
      (`/Engine/EditorBlueprintResources/StandardMacros.IsValid` _currentcrystal
        (:`Is Valid`
          (set `/Game/Puzzle_and_Trap/PuzzleParts/Laser_Puzzles/BP_Laser_Cube.Active` false _currentcrystal)
          (set `self.CurrentCrystal` (`self.noCrystal`)))))))

(fn `UserConstructionScript`
  (`parent.UserConstructionScript`))