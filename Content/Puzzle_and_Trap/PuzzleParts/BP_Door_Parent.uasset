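; BP_Door_Parent is a parent puzzle door that opens once all of its linked levers are activated.
; On BeginPlay it registers itself as the door on each lever in its ThisLever array.
; CallCheck_Event runs the CheckDoorActivation macro, which checks every valid lever, latches IsActivated and swings DoorHinge open to about -90 yaw, one step per tick.
; A CheckActivation function duplicates this logic with an instant, same-frame rotation loop.
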(event `self.ReceiveBeginPlay`
  ;[1 1 1] Lever pairing and check door call
  (for _array_element (`self.ThisLever`)
    (set `/Game/Puzzle_and_Trap/PuzzleParts/BP_Lever_Parent.ThisDoor` self _array_element)))

(event `CallCheck_Event`
  ;[1 1 1] Lever pairing and check door call
  (`self.CheckDoorActivation`))

(fn `CheckActivation`
  (bind _doorhinge (`self.DoorHinge`))
  (bind (_relativerotation_roll _relativerotation_pitch _relativerotation_yaw) (`KismetMathLibrary.BreakRotator` (`SceneComponent.RelativeRotation` _doorhinge)))
  (if (not (`self.IsActivated`))
    (set `self.IsActivated` true)
    (for _array_element (`self.ThisLever`)
      (`/Engine/EditorBlueprintResources/StandardMacros.IsValid` _array_element
        (:`Is Valid`
          (if (not (`/Game/Puzzle_and_Trap/PuzzleParts/BP_Lever_Parent.IsActivated` _array_element))
            (set `self.IsActivated` false)))))
    (while (and (`self.IsActivated`) (> _relativerotation_yaw -90.0))
      (`SceneComponent.K2_AddRelativeRotation` _doorhinge (struct :`Yaw` -5.0) false false))))

(fn `UserConstructionScript`)