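; Puzzle statue that acts as a lever for a linked door, activated by damage of the CocoChargedAttack type.
; A qualifying hit sets Active and, if DoorRef is valid, calls CheckToOpen on that door.
; The same valid-door branch then creates a dynamic Eyes material instance on the statue and sets EyeColor to black.
; Nothing here resets Active, and the collision box overlap event is empty.
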(event `self.ReceiveAnyDamage`
  (params (Damage :type "Float (single-precision)") (DamageType :type "DamageType Object Reference") (InstigatedBy :type "Controller Object Reference") (DamageCauser :type "Actor Object Reference"))
  (bind _doorref (`self.DoorRef`))
  ;[1 1 1] Statue activation and door check call
  (cast `/Game/CocoChargedAttack` DamageType)
  (set `self.Active` true)
  (`/Engine/EditorBlueprintResources/StandardMacros.IsValid` _doorref
    (:`Is Valid`
      (`/Game/Interactables/BP_LockedDoor.CheckToOpen` _doorref)
      (if (`self.Active`)
        (bind _returnvalue (`PrimitiveComponent.CreateDynamicMaterialInstance` (`self.Statue`) 0 "/Game/eyes.eyes" "None"))
        (`MaterialInstanceDynamic.SetVectorParameterValue` _returnvalue "EyeColor" (struct :`A` 1.0))))))

(event `self.coll box.OnComponentBeginOverlap`
  (params (OverlappedComponent :type "PrimitiveComponent Object Reference") (OtherActor :type "Actor Object Reference") (OtherComp :type "PrimitiveComponent Object Reference") (OtherBodyIndex :type Integer) (bFromSweep :type Boolean) (SweepResult :type "HitResult Structure (by ref)")))

(fn `UserConstructionScript`
  (`parent.UserConstructionScript`))