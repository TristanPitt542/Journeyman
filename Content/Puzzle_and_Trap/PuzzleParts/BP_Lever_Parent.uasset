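; Parent lever Blueprint for puzzle rooms that latches on when something overlaps its sphere and notifies a linked door.
; On overlap it sets IsActivated and, if ThisDoor is valid, calls the door's CallCheckEvent.
; It then pitches ShaftAnchor down in fixed steps, one per tick via a DelayUntilNextTick loop, until it reaches its limit.
; The shaft only animates when a door is linked, and nothing here resets the lever.
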(event `self.Sphere.OnComponentBeginOverlap`
  (params (OverlappedComponent :type "PrimitiveComponent Object Reference") (OtherActor :type "Actor Object Reference") (OtherComp :type "PrimitiveComponent Object Reference") (OtherBodyIndex :type Integer) (bFromSweep :type Boolean) (SweepResult :type "HitResult Structure (by ref)"))
  (bind _thisdoor (`self.ThisDoor`))
  (bind _shaftanchor (`self.ShaftAnchor`))
  (bind (_relativerotation_roll _relativerotation_pitch) (`KismetMathLibrary.BreakRotator` (`SceneComponent.RelativeRotation` _shaftanchor)))
  ;[1 1 1] Lever activation and door check call
  (set `self.IsActivated` true)
  (`/Engine/EditorBlueprintResources/StandardMacros.IsValid` _thisdoor
    (:`Is Valid`
      (`/Game/Puzzle_and_Trap/PuzzleParts/BP_Door_Parent.CallCheck_Event` _thisdoor)
      (if (and (`self.IsActivated`) (> _relativerotation_pitch -25.0)) :!label _label
        (`SceneComponent.K2_AddRelativeRotation` _shaftanchor (struct :`Pitch` -5.0) false false)
        (`KismetSystemLibrary.DelayUntilNextTick`)
        (goto _label)))))

(fn `UserConstructionScript`)