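; Base pickup item that spins on its yaw axis and flies toward the player (BP_Coco).
; Tick increments the root's yaw every frame, independent of delta time.
; A PickupRange overlap starts a timeline that lerps the item from its current location to Coco's live position, with sweep.
; If CanPickup is false or the actor isn't BP_Coco, the check retries every 0.2 seconds, even after the overlap ends.
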(event `self.ReceiveTick`
  (params (DeltaSeconds :type "Float (single-precision)"))
  (bind _defaultsceneroot (`self.DefaultSceneRoot`))
  (bind (_returnvalue_roll _returnvalue_pitch _returnvalue_yaw) (`KismetMathLibrary.BreakRotator` (`SceneComponent.K2_GetComponentRotation` _defaultsceneroot)))
  ;[1 1 1] Rotate
  (bind _result (`/Engine/EditorBlueprintResources/StandardMacros.IncrementFloat` _returnvalue_yaw)
    (:`  `
      (`SceneComponent.K2_SetWorldRotation` _defaultsceneroot (`KismetMathLibrary.MakeRotator` _returnvalue_roll _returnvalue_pitch _result) false false))))

(event `self.pickup range.OnComponentBeginOverlap`
  (params (OverlappedComponent :type "PrimitiveComponent Object Reference") (OtherActor :type "Actor Object Reference") (OtherComp :type "PrimitiveComponent Object Reference") (OtherBodyIndex :type Integer) (bFromSweep :type Boolean) (SweepResult :type "HitResult Structure (by ref)"))
  ;[1 1 1] Move towards player
  (if (and (`self.CanPickup`) (== (`GameplayStatics.GetObjectClass` OtherActor) "/Game/CharacterController/BP_Coco.BP_Coco_C")) :!label _label
    (bind _asbp_coco (cast `/Game/CharacterController/BP_Coco` OtherActor))
    (bind (_direction _newtrack_0) (`Timeline|MoveToCoco` :!via `PlayFromStart`)
      (:`Update`
        (`self.K2_SetActorLocation` (`KismetMathLibrary.VLerp` (`self.K2_GetActorLocation`) (`self.K2_GetActorLocation` _asbp_coco) _newtrack_0) true)))
    (else
      (`KismetSystemLibrary.Delay` 0.2)
      (goto _label))))

(fn `UserConstructionScript`)