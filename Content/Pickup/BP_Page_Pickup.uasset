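; BP_Page_Pickup is a collectible page that adds a page to the player's manual.
; When the Page component is overlapped by an actor of class BP_Coco, it casts player controller 0's HUD to BP_UI and calls AddManualPage.
; The pickup then destroys itself; if the HUD cast fails, it stays in place.
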(event `self.Page.OnComponentBeginOverlap`
  (params (OverlappedComponent :type "PrimitiveComponent Object Reference") (OtherActor :type "Actor Object Reference") (OtherComp :type "PrimitiveComponent Object Reference") (OtherBodyIndex :type Integer) (bFromSweep :type Boolean) (SweepResult :type "HitResult Structure (by ref)"))
  ;[1 1 1] Adds the page to the players manual when overlapped
  (if (== (`GameplayStatics.GetObjectClass` OtherActor) "/Game/CharacterController/BP_Coco.BP_Coco_C")
    (bind _asbp_ui (cast `/Game/UI/Widgets/BP_UI` (`PlayerController.GetHUD` (`GameplayStatics.GetPlayerController` 0))))
    (`/Game/UI/Widgets/BP_UI.Add Manual Page` _asbp_ui)
    (`self.K2_DestroyActor`)))

(fn `UserConstructionScript`
  (`parent.UserConstructionScript`))