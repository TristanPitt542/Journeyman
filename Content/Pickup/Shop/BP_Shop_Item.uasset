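; BP_Shop_Item is a shop pickup that Coco can buy with Money through its Interact event.
; Overlapping its Box shows a Prompt and disables dashing on the Coco controller until the player leaves.
; Interact calls Purchase when Money covers Price, which deducts the cost, refreshes the BP_UI item counts and destroys the actor.
; Purchase itself grants no item, only passing Coco's current Holy Water and Garlic Bomb counts to the HUD.
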(event `self.ReceiveBeginPlay`
  (bind _asbp_coco_controller (cast `/Game/CharacterController/BP_Coco_Controller` (`GameplayStatics.GetPlayerController` 0)))
  (set `self.As BP Coco Controller` _asbp_coco_controller)
  (bind _asbp_coco (cast `/Game/CharacterController/BP_Coco` (`GameplayStatics.GetPlayerPawn` 0)))
  (set `self.As BP Coco` _asbp_coco))

(event `self.Box.OnComponentBeginOverlap`
  (params (OverlappedComponent :type "PrimitiveComponent Object Reference") (OtherActor :type "Actor Object Reference") (OtherComp :type "PrimitiveComponent Object Reference") (OtherBodyIndex :type Integer) (bFromSweep :type Boolean) (SweepResult :type "HitResult Structure (by ref)"))
  (if (== (`GameplayStatics.GetObjectClass` OtherActor) "/Game/CharacterController/BP_Coco.BP_Coco_C")
    (`SceneComponent.SetVisibility` (`self.Prompt`) true false)
    (set `/Game/CharacterController/BP_Coco_Controller.CanDash` false (`self.As BP Coco Controller`))))

(event `self.Box.OnComponentEndOverlap`
  (params (OverlappedComponent :type "PrimitiveComponent Object Reference") (OtherActor :type "Actor Object Reference") (OtherComp :type "PrimitiveComponent Object Reference") (OtherBodyIndex :type Integer))
  (if (== (`GameplayStatics.GetObjectClass` OtherActor) "/Game/CharacterController/BP_Coco.BP_Coco_C")
    (`SceneComponent.SetVisibility` (`self.Prompt`) false false)
    (set `/Game/CharacterController/BP_Coco_Controller.CanDash` true (`self.As BP Coco Controller`))))

(event `/Game/Interactables/BPI_Interact.Interact`
  (if (>= (`/Game/CharacterController/BP_Coco.Money` (`self.As BP Coco`)) (`self.Price`))
    (`self.Purchase`)))

(fn `Purchase`
  (bind _as_bp_coco (`self.As BP Coco`))
  (bind _as_bp_coco_2 (`self.As BP Coco`))
  (set `/Game/CharacterController/BP_Coco.Money` (- (`/Game/CharacterController/BP_Coco.Money` _as_bp_coco) (`self.Price`)) _as_bp_coco)
  (bind _asbp_ui (cast `/Game/UI/Widgets/BP_UI` (`PlayerController.GetHUD` (`GameplayStatics.GetPlayerController` 0))))
  (`/Game/UI/Widgets/BP_UI.Update Item Count` _asbp_ui (`/Game/CharacterController/BP_Coco.Holy Water Count` _as_bp_coco_2) (`/Game/CharacterController/BP_Coco.Garlic Bomb Count` _as_bp_coco_2) -1)
  (`self.K2_DestroyActor`))

(fn `UserConstructionScript`)